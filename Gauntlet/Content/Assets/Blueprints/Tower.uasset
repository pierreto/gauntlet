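; Tower actor that continuously spins its static mesh around the local X (roll) axis at a randomized rate and direction.
; On BeginPlay it rerolls a random integer from -2 to 2 until it is non-zero, then starts a looping timer.
; Each timer tick adds a local rotation of that integer times RotationSpeed, scaled by the timer interval so speed stays independent of the interval.
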(event `self.ReceiveBeginPlay`
  (bind _output_get (set `self.Random_Int` (`KismetMathLibrary.RandomIntegerInRange` -2 2) :!label _label))
  (if (== _output_get 0)
    (goto _label)
    (else
      (`KismetSystemLibrary.K2_SetTimerDelegate` (delegate `Rotate_Ring_01`) (`self.Time`) true))))

(event `Rotate_Ring_01`
  (`SceneComponent.K2_AddLocalRotation` (`self.StaticMesh`) (* (`KismetMathLibrary.MakeRotator` (* (`self.Random_Int`) (`self.RotationSpeed`))) (`self.Time`)) false false))

(fn `UserConstructionScript`)