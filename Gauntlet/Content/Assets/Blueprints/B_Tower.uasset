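; B_Tower is a tower Blueprint that continuously spins three static mesh components around their yaw axis.
; BeginPlay starts a looping timer, with no Tick logic, that rotates all three meshes on each firing.
; The first turns at the base speed, the second in the opposite direction and the third at half speed.
; Each step scales RotationSpeed by the timer interval Time, making it a per-second rate.
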(event `self.ReceiveBeginPlay`
  (`KismetSystemLibrary.K2_SetTimerDelegate` (delegate `Rotate_Ring_01`) (`self.Time`) true))

(event `Rotate_Ring_01`
  (bind _returnvalue (* (`KismetMathLibrary.MakeRotator` 0.0 0.0 (`self.RotationSpeed`)) (`self.Time`)))
  (`|ExecutionSequence`
    (:`then_0`
      (`SceneComponent.K2_AddLocalRotation` (`self.StaticMesh_01`) _returnvalue false false))
    (:`then_1`
      (`SceneComponent.K2_AddLocalRotation` (`self.StaticMesh_02`) (* _returnvalue -1) false false))
    (:`then_2`
      (`SceneComponent.K2_AddLocalRotation` (`self.StaticMesh_03`) (* _returnvalue 0.5) false false))))

(fn `UserConstructionScript`)