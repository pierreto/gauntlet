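; Rotating ring Blueprint that spins its static mesh continuously around a randomly chosen combination of axes.
; On BeginPlay it re-rolls two small random integers until both are non-zero, setting a direction and speed multiplier for roll and pitch.
; A looping timer, used in place of Tick, then adds local rotation scaled by RotationSpeed and the timer interval, leaving yaw untouched.
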(event `self.ReceiveBeginPlay`
  (bind _output_get (set `self.Random_Int` (`KismetMathLibrary.RandomIntegerInRange` -2 2) :!label _label))
  (if (== _output_get 0)
    (goto _label)
    (else
      (bind _output_get_2 (set `self.Random_Int_0` (`KismetMathLibrary.RandomIntegerInRange` -2 2) :!label _label_2))
      (if (== _output_get_2 0)
        (goto _label_2)
        (else
          (`KismetSystemLibrary.K2_SetTimerDelegate` (delegate `Rotate_Ring_01`) (`self.Time`) true))))))

(event `Rotate_Ring_01`
  (bind _rotationspeed (`self.RotationSpeed`))
  (`SceneComponent.K2_AddLocalRotation` (`self.StaticMesh`) (* (`KismetMathLibrary.MakeRotator` (* (`self.Random_Int`) _rotationspeed) (* (`self.Random_Int_0`) _rotationspeed)) (`self.Time`)) false false))

(fn `UserConstructionScript`)