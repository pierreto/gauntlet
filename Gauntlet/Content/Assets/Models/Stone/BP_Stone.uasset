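; Stone actor that appears, flies to the right hand of a BP_Hands actor and then rotates around it.
; Start stores the target and spin speed, multicasts the endgame particle, then reveals the stone after a short delay.
; Tick, on authority only, accelerates it toward the hand skeleton up to a max speed.
; On arrival it offsets the stone, attaches to the skeleton and hands motion to RotatingMovement.
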(event `self.ReceiveTick`
  (params (DeltaSeconds :type "Float (single-precision)"))
  (bind _returnvalue (- (`SceneComponent.K2_GetComponentLocation` (`/Game/Blueprints/GestureSpells/Hand.HandSkeleton` (`self.FollowTarget`))) (`self.K2_GetActorLocation`)))
  ;[1 1 1] Go to hand and attach to it
  (`/Engine/EditorBlueprintResources/ActorMacros.Switch Has Authority`
    (:`Authority`
      (if (`self.Moving?`)
        (`/Engine/EditorBlueprintResources/StandardMacros.IsValid` (`self.FollowTarget`)
          (:`Is Valid`
            (if (>= (`KismetMathLibrary.VSize` _returnvalue) 1.0)
              (`self.K2_AddActorWorldOffset` (* (`KismetMathLibrary.Normal` _returnvalue) (* DeltaSeconds (`self.GetSpeed` DeltaSeconds))))
              (else
                (set `self.CurrentSpeed` 0.0)
                ;;[1 1 1] Reached the hand, start rotating around it
                (`SceneComponent.K2_AddRelativeLocation` (`self.Stone`) (30.0 0.0 0.0) false false)
                (`self.K2_AttachToComponent` (`/Game/Blueprints/GestureSpells/Hand.HandSkeleton` (`self.FollowTarget`)) "None" "SnapToTarget" "SnapToTarget" "SnapToTarget")
                (set `RotatingMovementComponent.RotationRate` (`KismetMathLibrary.MakeRotator` 0.0 (`self.RotationSpeed`)) (`self.RotatingMovement`))
                (set `self.Moving?` false)))))))))

(event `Start`
  (params (Actor :type "Actor Object Reference") (Speed :type "Float (double-precision)" :default 90.0))
  (set `self.RotationSpeed` Speed)
  (bind _asbp_hands (cast `/Game/Blueprints/Characters/BP_Hands` Actor))
  (set `self.FollowTarget` (`/Game/Blueprints/Characters/BP_Hands.HandR` _asbp_hands))
  (`self.PlayParticleMulticast`)
  (`KismetSystemLibrary.Delay` 2.0)
  (`SceneComponent.SetVisibility` (`self.Stone`) true false)
  (set `self.Moving?` true))

(event `PlayParticleMulticast`
  (`ActorComponent.Activate` (`self.Endgame_P`) false))

(fn `GetDestination`
  (returns (Destination :type "Vector Structure"))
  (locals (HandDestination :type "Vector Structure"))
  (bind _followtarget (`self.FollowTarget`))
  (`/Engine/EditorBlueprintResources/StandardMacros.IsValid` (`self.FollowTarget`)
    (:`Is Valid`
      (set `local.HandDestination` (+ (`/Game/Blueprints/GestureSpells/Hand.GetHandCenter` _followtarget) (* (`/Game/Blueprints/GestureSpells/Hand.GetPalmVector` _followtarget) 20.0))))
    (:`Is Not Valid`
      (set `local.HandDestination` (`self.K2_GetActorLocation`))))
  (return (`local.HandDestination`)))

(fn `GetSpeed`
  (params (DeltaTime :type "Float (double-precision)"))
  (returns (Speed :type "Float (double-precision)"))
  (if (not (>= (`self.CurrentSpeed`) (`self.MaxFollowSpeed`)))
    (bind _output_get (set `self.CurrentSpeed` (+ (`self.CurrentSpeed`) (* DeltaTime (`self.FollowAcceleration`))))))
  (return _output_get))

(fn `UpdatePivotPoint`
  (set `RotatingMovementComponent.PivotTranslation` (`KismetMathLibrary.InverseTransformDirection` (`SceneComponent.K2_GetComponentToWorld` (`self.DefaultSceneRoot`)) (- (`self.K2_GetActorLocation` (`self.Target`)) (`self.K2_GetActorLocation`))) (`self.RotatingMovement`)))

(fn `UserConstructionScript`)