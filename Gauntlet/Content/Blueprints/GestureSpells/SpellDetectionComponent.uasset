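; Component that runs gesture spell detection by polling the BP_Spell actors in the level with left and right hand input.
; BeginPlay caches all spell actors, and Tick offers both hands to each one's InitialDetection until the first match becomes the current spell.
; While a spell is current, only its Detect runs each frame with delta time, and a true result clears it so scanning resumes.
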(event `self.ReceiveBeginPlay`
  ;[1 1 1] Get All Spells
  (bind _outactors (`GameplayStatics.GetAllActorsOfClass` "/Game/Blueprints/GestureSpells/Spells/BP_Spell.BP_Spell_C"))
  (set `self.Spells` _outactors))

(event `self.ReceiveTick`
  (params (DeltaSeconds :type "Float (single-precision)"))
  ;[1 1 1] Main Detection Loop
  (`/Engine/EditorBlueprintResources/StandardMacros.IsValid` (`self.CurrentSpell`)
    (:`Is Valid`
      (bind _detected (`/Game/Blueprints/GestureSpells/Spells/BP_Spell.Detect` (`self.CurrentSpell`) (`self.LeftHand`) (`self.RightHand`) DeltaSeconds))
      (if _detected
        (set `self.CurrentSpell` null)))
    (:`Is Not Valid`
      (for _array_element (`self.Spells`)
        (bind _detected_2 (`/Game/Blueprints/GestureSpells/Spells/BP_Spell.InitialDetection` _array_element (`self.LeftHand`) (`self.RightHand`)))
        (if _detected_2
          (set `self.CurrentSpell` _array_element)
          (break))))))