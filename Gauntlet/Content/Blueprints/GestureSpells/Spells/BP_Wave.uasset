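; BP_Wave is a placeholder Wave gesture spell that implements initial and ongoing detection hooks for two hands, with no real gesture recognition yet.
; InitialDetection prints the spell's name and always succeeds.
; Detect ignores both hands and accumulates delta time, returning true and resetting the timer once five seconds have built up.
; The event graph holds only disabled default events, and no spell effect is defined here.
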(fn `Detect`
  (params (LeftHand :type "/Game/Blueprints/GestureSpells/Hand Object Reference") (RightHand :type "/Game/Blueprints/GestureSpells/Hand Object Reference") (DeltaTime :type "Float (double-precision)"))
  (returns (Detected :type Boolean))
  (locals (_detected :type Boolean))
  (bind _output_get (set `self.Time` (+ DeltaTime (`self.Time`))))
  (bind _output_get_2 (set `local._detected` (>= _output_get 5.0)))
  (if _output_get_2
    (set `self.Time` 0.0))
  (return (`local._detected`)))

(fn `InitialDetection`
  (params (LeftHand :type "/Game/Blueprints/GestureSpells/Hand Object Reference") (RightHand :type "/Game/Blueprints/GestureSpells/Hand Object Reference"))
  (returns (Detected :type Boolean))
  (`KismetSystemLibrary.PrintString` "BP_Wave")
  (return true))

(fn `UserConstructionScript`
  (`parent.UserConstructionScript`))