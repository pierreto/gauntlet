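; BP_Fireball is a gravity-free spell projectile, launched through SetVelocity along a given direction at its Speed.
; At construction it records which side of world Y=0 it spawned on, using that as its team.
; Overlapping opposing fireballs or actors destroys it and applies damage.
; An opposing BP_Shield instead reflects it along the shield's negated up vector at unchanged speed, flips its side and still takes damage.
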(event `self.ReceiveActorBeginOverlap`
  (params (OtherActor :type "Actor Object Reference"))
  (bind _projectilemovement (`self.ProjectileMovement`))
  (bind (_returnvalue_x _returnvalue_y) (`KismetMathLibrary.BreakVector` (`SceneComponent.K2_GetComponentLocation` (`Actor.RootComponent` OtherActor))))
  (bind _returnvalue (== (< _returnvalue_y 0.0) (`self.YInferior0`)))
  ;[1 1 1] Collision boule de feu
  (bind _asbp_fireball (cast `/Game/Blueprints/GestureSpells/Spells/BP_Fireball` OtherActor)
    (:`then`
      (if (not (== (`self.YInferior0`) (`/Game/Blueprints/GestureSpells/Spells/BP_Fireball.YInferior0` _asbp_fireball)))
        (`self.K2_DestroyActor` :!label _label)
        (`GameplayStatics.ApplyDamage` OtherActor 1.0 :!label _label_2)))
    (:`CastFailed`
      (bind _asbp_shield (cast `/Game/Blueprints/GestureSpells/Spells/BP_Shield` OtherActor)
        (:`then`
          (if (not _returnvalue)
            (set `MovementComponent.Velocity` (* (* (`SceneComponent.GetUpVector` (`/Game/Blueprints/GestureSpells/Spells/BP_Shield.Shield` _asbp_shield)) (`KismetMathLibrary.VSize` (`MovementComponent.Velocity` _projectilemovement))) -1) _projectilemovement)
            (set `self.YInferior0` (not (`self.YInferior0`)))
            (goto _label_2)))
        (:`CastFailed`
          (if (not _returnvalue)
            (goto _label)))))))

(event `SetVelocity`
  (params (Direction :type "Vector Structure"))
  ;[1 1 1] Lancer la fireball
  (set `MovementComponent.Velocity` (* Direction (`self.Speed`)) (`self.ProjectileMovement`)))

(fn `UserConstructionScript`
  (bind (_returnvalue_x _returnvalue_y) (`KismetMathLibrary.BreakVector` (`SceneComponent.K2_GetComponentLocation` (`self.Fire Ball`))))
  (set `self.YInferior0` (< _returnvalue_y 0.0))
  (set `ProjectileMovementComponent.ProjectileGravityScale` 0.0 (`self.ProjectileMovement`)))