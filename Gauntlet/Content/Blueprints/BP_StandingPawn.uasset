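; BP_StandingPawn is a standing VR pawn with a floor tracking origin, a toggleable menu and LAN multiplayer hosting and joining.
; ShowWidget input either destroys the visible menu or spawns a BP_MenuActor offset from the VR camera, facing it and attached to it.
; Host input creates a LAN session and opens Gym as a listen server.
; Join input searches LAN sessions and joins the first found, printing the result.
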(event `InputAction|ShowWidget`
  (params (Key :type "Key Structure"))
  (bind _menuwidget (`self.MenuWidget`))
  (:`Pressed`
    (`/Engine/EditorBlueprintResources/StandardMacros.IsValid` _menuwidget
      (:`Is Valid`
        (if (`SceneComponent.IsVisible` (`/Game/Blueprints/Widgets/BP_MenuActor.Widget` _menuwidget))
          (`self.HideMenuWidget`)
          (else
            (`self.ShowMenuWidget` :!label _label))))
      (:`Is Not Valid`
        (goto _label)))))

(event `self.ReceiveBeginPlay`
  (`HeadMountedDisplayFunctionLibrary.SetTrackingOrigin` "Floor"))

(event `HideMenuWidget`
  (bind _menuwidget (`self.MenuWidget`))
  (`/Engine/EditorBlueprintResources/StandardMacros.IsValid` _menuwidget
    (:`Is Valid`
      (if (`SceneComponent.IsVisible` (`/Game/Blueprints/Widgets/BP_MenuActor.Widget` _menuwidget))
        (`self.K2_DestroyActor` _menuwidget)
        (set `self.MenuWidget` null)))))

(event `InputAction|Host`
  (params (Key :type "Key Structure"))
  (:`Pressed`
    (`CreateSessionCallbackProxy.CreateSession` (`GameplayStatics.GetPlayerController` 0) 10 true
      (:`OnSuccess`
        (`GameplayStatics.OpenLevel` "Gym" true "Listen"))
      (:`OnFailure`
        (`KismetSystemLibrary.PrintString` "Failed")))))

(event `InputAction|Join`
  (params (Key :type "Key Structure"))
  (:`Pressed`
    (bind _results (`FindSessionsCallbackProxy.FindSessions` (`GameplayStatics.GetPlayerController` 0) 10 true)
      (:`OnSuccess`
        (if (`KismetArrayLibrary.Array_IsValidIndex` _results)
          (`JoinSessionCallbackProxy.JoinSession` (`GameplayStatics.GetPlayerController` 0) (`|GetArrayItem` _results)
            (:`OnSuccess`
              (`KismetSystemLibrary.PrintString` "SUCCESSSSS" true true (struct :`G` 0.66 :`B` 1.0 :`A` 1.0) 10.0))
            (:`OnFailure`
              (`KismetSystemLibrary.PrintString` "FAILUREEEE :(((((" true true (struct :`G` 0.66 :`B` 1.0 :`A` 1.0) 10.0)))))
      (:`OnFailure`
        (`KismetSystemLibrary.PrintString` "Error while trying to find sessions")))))

(fn `ShowMenuWidget`
  (bind _returnvalue_roll (`KismetMathLibrary.BreakRotator` (`self.K2_GetActorRotation`)))
  (bind _vrcamera (`self.VRCamera`))
  (bind (_returnvalue_roll_2 _returnvalue_pitch _returnvalue_yaw) (`KismetMathLibrary.BreakRotator` (`SceneComponent.K2_GetComponentRotation` _vrcamera)))
  (bind _returnvalue (`KismetMathLibrary.MakeRotator` 0.0 _returnvalue_pitch _returnvalue_yaw))
  (bind (_returnvalue_roll_3 _returnvalue_pitch_2 _returnvalue_yaw_2) (`KismetMathLibrary.BreakRotator` (`KismetMathLibrary.FindLookAtRotation` (`self.K2_GetActorLocation` (`self.MenuWidget`)) (`SceneComponent.K2_GetComponentLocation` (`self.VRCamera`)))))
  (bind _returnvalue_2 (`|SpawnActorFromClass` "/Game/Blueprints/Widgets/BP_MenuActor.BP_MenuActor_C" (`KismetMathLibrary.MakeTransform` (0.0 0.0 0.0) (struct) (0.1 0.1 0.1)) "Undefined" "OverrideRootScale" null null))
  (bind _asbp_menu_actor (cast `/Game/Blueprints/Widgets/BP_MenuActor` _returnvalue_2))
  (bind _output_get (set `self.MenuWidget` _asbp_menu_actor))
  (`self.K2_SetActorLocation` _output_get (+ (`SceneComponent.K2_GetComponentLocation` _vrcamera) (+ (* (`KismetMathLibrary.GetForwardVector` _returnvalue) (`self.ForwardDistance`)) (* (`KismetMathLibrary.GetUpVector` _returnvalue) (`self.UpDistance`)))) false false)
  (`self.K2_SetActorRotation` _output_get (`KismetMathLibrary.MakeRotator` _returnvalue_roll _returnvalue_pitch_2 _returnvalue_yaw_2) false)
  (if (`.ReturnValue` (`NavigationSystemV1.K2_ProjectPointToNavigation` (`SceneComponent.K2_GetComponentLocation` (`/Game/Blueprints/Widgets/BP_MenuActor.Widget` (`self.MenuWidget`)))))
    _
    (else
      _))
  (`SceneComponent.SetVisibility` (`/Game/Blueprints/Widgets/BP_MenuActor.Widget` (`self.MenuWidget`)) true false)
  (`self.K2_AttachToComponent` (`self.MenuWidget`) (`self.VRCamera`) "None" "KeepWorld" "KeepWorld" "KeepWorld" false))

(fn `UserConstructionScript`)