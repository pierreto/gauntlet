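; BP_Pray is an input-driven actor that starts or joins LAN multiplayer sessions and sets the VR tracking origin to floor level on BeginPlay.
; The Host input creates a LAN session and, on success, opens the Gym level as a listen server.
; The Join input searches for LAN sessions and joins the first result, with on-screen prints reporting progress and most failures.
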(event `self.ReceiveBeginPlay`
  (`HeadMountedDisplayFunctionLibrary.SetTrackingOrigin` "Floor"))

(event `InputAction|Host`
  (params (Key :type "Key Structure"))
  (:`Pressed`
    (`KismetSystemLibrary.PrintString` "HOST PRESSED" true true (struct :`G` 0.66 :`B` 1.0 :`A` 1.0) 5.0)
    (`CreateSessionCallbackProxy.CreateSession` (`GameplayStatics.GetPlayerController` 0) 10 true
      (:`OnSuccess`
        (`GameplayStatics.OpenLevel` "Gym" true "Listen"))
      (:`OnFailure`
        (`KismetSystemLibrary.PrintString` "Failed")))))

(event `InputAction|Join`
  (params (Key :type "Key Structure"))
  (:`Pressed`
    (`KismetSystemLibrary.PrintString` "JOIN PRESSED" true true (struct :`G` 0.66 :`B` 1.0 :`A` 1.0) 5.0)
    (bind _results (`FindSessionsCallbackProxy.FindSessions` (`GameplayStatics.GetPlayerController` 0) 10 true)
      (:`OnSuccess`
        (if (`KismetArrayLibrary.Array_IsValidIndex` _results)
          (`JoinSessionCallbackProxy.JoinSession` (`GameplayStatics.GetPlayerController` 0) (`|GetArrayItem` _results)
            (:`OnSuccess`
              (`KismetSystemLibrary.PrintString` "SUCCESSSSS" true true (struct :`G` 0.66 :`B` 1.0 :`A` 1.0) 10.0))
            (:`OnFailure`
              (`KismetSystemLibrary.PrintString` "FAILUREEEE :(((((" true true (struct :`G` 0.66 :`B` 1.0 :`A` 1.0) 10.0)))))
      (:`OnFailure`
        (`KismetSystemLibrary.PrintString` "Error while trying to find sessions")))))

(fn `UserConstructionScript`)