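; BP_HitIndicator is a short-lived effect actor that drifts a sphere away from its spawn point while fading it out.
; Construction picks a random direction within a 60-degree half-angle cone around world up.
; Each tick it moves along that direction at a speed sampled from a curve over normalized lifetime, scaled by SpeedFactor.
; The sphere material's Opacity parameter falls linearly over Duration, then the actor destroys itself.
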(event `self.ReceiveTick`
  (params (DeltaSeconds :type "Float (single-precision)"))
  ;[1 1 1] Move and fade over duration
  (set `self.CurrentTime` (+ DeltaSeconds (`self.CurrentTime`)))
  (`self.Move` DeltaSeconds)
  (`self.Fade`)
  ;[1 1 1] Destroy when done
  (if (>= (`self.CurrentTime`) (`self.Duration`))
    (`self.K2_DestroyActor`)))

(fn `Fade`
  (`MeshComponent.SetScalarParameterValueOnMaterials` (`self.Sphere`) "Opacity" (- 1.0 (/ (`self.CurrentTime`) (`self.Duration`)))))

(fn `GetSpeed`
  (returns (Speed :type "Float (double-precision)"))
  (return (`CurveFloat.GetFloatValue` (`self.SpeedCurve`) (/ (`self.CurrentTime`) (`self.Duration`)))))

(fn `Move`
  (params (DeltaTime :type "Float (double-precision)"))
  (`self.K2_AddActorWorldOffset` (* (`self.Direction`) (* (`self.GetSpeed`) DeltaTime (`self.SpeedFactor`)))))

(fn `UserConstructionScript`
  (set `self.Direction` (`KismetMathLibrary.RandomUnitVectorInConeInDegrees` (0.0 0.0 1.0) 60.0)))