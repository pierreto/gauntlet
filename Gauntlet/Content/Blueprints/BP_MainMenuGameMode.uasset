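; Main menu game mode that handles hosting and joining LAN multiplayer sessions.
; HostGame creates a LAN session and, on success, opens the Gym level as a listen server.
; JoinGame searches for LAN sessions and joins the first valid result without offering a choice.
; Failed session creation or search only prints an error string.
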(event `HostGame`
  (`CreateSessionCallbackProxy.CreateSession` (`GameplayStatics.GetPlayerController` 0) 10 true
    (:`OnSuccess`
      (`GameplayStatics.OpenLevel` "Gym" true "Listen"))
    (:`OnFailure`
      (`KismetSystemLibrary.PrintString` "Failed"))))

(event `JoinGame`
  (bind _results (`FindSessionsCallbackProxy.FindSessions` null 10 true)
    (:`OnSuccess`
      (if (`KismetArrayLibrary.Array_IsValidIndex` _results)
        (`JoinSessionCallbackProxy.JoinSession` (`GameplayStatics.GetPlayerController` 0) (`|GetArrayItem` _results))))
    (:`OnFailure`
      (`KismetSystemLibrary.PrintString` "Error while trying to find sessions"))))

(fn `UserConstructionScript`)