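; Menu actor that relays pointer hits and trigger presses to the MainMenu widget hosted in its widget component.
; RaytraceWorldLocation converts a world location into the component's local space with an inverse transform, negates it and passes it to the widget's RaytraceWidgetLocation.
; TriggerPressedOnMenu forwards a press to the widget's ButtonClicked, leaving the response to the widget itself.
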(event `RaytraceWorldLocation`
  (params (Location :type "Vector Structure"))
  (bind _mainmenuwidget (`self.MainMenuWidget`))
  ;[1 1 1] World Space To Widget Space
  (bind _asmain_menu (cast `/Game/Blueprints/MainMenu` (`WidgetComponent.GetUserWidgetObject` _mainmenuwidget)))
  (`/Game/Blueprints/MainMenu.RaytraceWidgetLocation` _asmain_menu (* (`KismetMathLibrary.InverseTransformLocation` (`SceneComponent.K2_GetComponentToWorld` _mainmenuwidget) Location) -1)))

(event `TriggerPressedOnMenu`
  ;[1 1 1] Trigger Pressed
  (bind _asmain_menu (cast `/Game/Blueprints/MainMenu` (`WidgetComponent.GetUserWidgetObject` (`self.MainMenuWidget`))))
  (`/Game/Blueprints/MainMenu.ButtonClicked` _asmain_menu))

(fn `UserConstructionScript`)