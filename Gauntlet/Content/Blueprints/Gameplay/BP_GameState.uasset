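; BP_GameState is a game state Blueprint that holds the match phase and a countdown timer.
; BeginPlay sets an initial phase, and StartCountdown sets the timer value without changing the phase.
; Tick calls CountdownTick, which decreases the timer only during one specific phase.
; When the timer runs out it is clamped to zero, and only the authority advances GameState to the next phase.
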(event `self.ReceiveBeginPlay`
  (set `self.GameState` "NewEnumerator3"))

(event `self.ReceiveTick`
  (params (DeltaSeconds :type "Float (single-precision)"))
  (`self.CountdownTick` DeltaSeconds))

(event `StartCountdown`
  (params (Countdown :type "Float (double-precision)"))
  ;[1 1 1] Start countdown
  (set `self.Countdown` Countdown))

(fn `CountdownTick`
  (params (DeltaTime :type "Float (double-precision)"))
  ;[1 1 1] Decrease countdown
  (if (`|EnumEquality` (`self.GameState`) "NewEnumerator4")
    (if (> (`self.Countdown`) 0.1)
      (set `self.Countdown` (- (`self.Countdown`) DeltaTime))
      (else
        ;[1 1 1] Check when countdown ends on server
        (set `self.Countdown` 0.0)
        (`/Engine/EditorBlueprintResources/ActorMacros.Switch Has Authority`
          (:`Authority`
            (set `self.GameState` "NewEnumerator1")))))))

(fn `UserConstructionScript`)