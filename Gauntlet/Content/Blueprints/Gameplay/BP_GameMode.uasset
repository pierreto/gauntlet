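; Multiplayer game mode that spawns and possesses a character for each joining player and gates match start on a full player count.
; On login, the server re-queries PlayerStart actors, spawns BP_Character at the one indexed by the running player counter, then increments it.
; ReadyToStartMatch returns true only when the player count equals MaxPlayerCount.
; The PlayerStart array cached on BeginPlay is not used by the login spawn.
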(event `self.ReceiveBeginPlay`
  ;[1 1 1] Begin and Get All PlayerStart
  (`/Engine/EditorBlueprintResources/ActorMacros.Switch Has Authority`
    (:`Authority`
      (bind _outactors (`GameplayStatics.GetAllActorsOfClass` "/Script/Engine.PlayerStart"))
      (set `self.PlayerStartArray` _outactors))))

(event `self.K2_PostLogin`
  (params (NewPlayer :type "PlayerController Object Reference"))
  ;[1 1 1] When a player joins game
  (`/Engine/EditorBlueprintResources/ActorMacros.Switch Has Authority`
    (:`Authority`
      (bind _outactors (`GameplayStatics.GetAllActorsOfClass` "/Script/Engine.PlayerStart"))
      (bind _returnvalue (`|SpawnActorFromClass` "/Game/Blueprints/Characters/BP_Character.BP_Character_C" (`self.GetTransform` (`|GetArrayItem` _outactors (`self.PlayersIngame`))) "AdjustIfPossibleButAlwaysSpawn" "OverrideRootScale" null null))
      (`Controller.Possess` NewPlayer _returnvalue)
      (`/Engine/EditorBlueprintResources/StandardMacros.IncrementInt` (`self.PlayersIngame`)))))

(fn `ReadyToStartMatch`
  (returns (ReturnValue :type Boolean))
  (bind _returnvalue (`self.GetNumPlayers`))
  (return (== _returnvalue (`self.MaxPlayerCount`))))

(fn `UserConstructionScript`)