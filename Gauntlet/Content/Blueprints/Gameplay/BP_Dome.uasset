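; BP_Dome is a dome that shows expanding bounce effects at given hit positions through its sphere's dynamic material.
; DoBounceEffect uses nested FlipFlops to rotate through four material slots, so successive hits can animate simultaneously.
; Each slot sets its own hit position vector and restarts its own timeline, which drives that slot's radius parameter scaled by BounceEffectRadius.
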(event `DoBounceEffect`
  (params (HitPos :type "Vector Structure"))
  (bind _returnvalue (`PrimitiveComponent.CreateDynamicMaterialInstance` (`self.Sphere1`) 0 null "None"))
  (set `self.MaterialInstance` _returnvalue)
  (set `self.HitPos` (`KismetMathLibrary.Conv_VectorToLinearColor` HitPos))
  (`/Engine/EditorBlueprintResources/StandardMacros.FlipFlop`
    (:`A`
      (`/Engine/EditorBlueprintResources/StandardMacros.FlipFlop`
        (:`A`
          (`MaterialInstanceDynamic.SetVectorParameterValue` (`self.MaterialInstance`) "HitPos0" (`self.HitPos`))
          (bind (_direction _newtrack_0) (`Timeline|Timeline` :!via `PlayFromStart`)
            (:`Update`
              (`MaterialInstanceDynamic.SetScalarParameterValue` (`self.MaterialInstance`) "Radius0" (* _newtrack_0 (`self.BounceEffectRadius`))))))
        (:`B`
          (`MaterialInstanceDynamic.SetVectorParameterValue` (`self.MaterialInstance`) "HitPos1" (`self.HitPos`))
          (bind (_direction_2 _newtrack_0_2) (`Timeline|Timeline_0` :!via `PlayFromStart`)
            (:`Update`
              (`MaterialInstanceDynamic.SetScalarParameterValue` (`self.MaterialInstance`) "Radius1" (* _newtrack_0_2 (`self.BounceEffectRadius`))))))))
    (:`B`
      (`/Engine/EditorBlueprintResources/StandardMacros.FlipFlop`
        (:`A`
          (`MaterialInstanceDynamic.SetVectorParameterValue` (`self.MaterialInstance`) "HitPos2" (`self.HitPos`))
          (bind (_direction_3 _newtrack_0_3) (`Timeline|Timeline_1` :!via `PlayFromStart`)
            (:`Update`
              (`MaterialInstanceDynamic.SetScalarParameterValue` (`self.MaterialInstance`) "Radius2" (* _newtrack_0_3 (`self.BounceEffectRadius`))))))
        (:`B`
          (`MaterialInstanceDynamic.SetVectorParameterValue` (`self.MaterialInstance`) "HitPos3" (`self.HitPos`))
          (bind (_direction_4 _newtrack_0_4) (`Timeline|Timeline_2` :!via `PlayFromStart`)
            (:`Update`
              (`MaterialInstanceDynamic.SetScalarParameterValue` (`self.MaterialInstance`) "Radius3" (* _newtrack_0_4 (`self.BounceEffectRadius`))))))))))

(fn `UserConstructionScript`)