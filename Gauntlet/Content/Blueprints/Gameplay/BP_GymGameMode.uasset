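; Game mode for a multiplayer gym match that spawns players as BP_Hands, runs the game phases and detects defeat.
; PostLogin spawns and possesses a pawn at one of two PlayerStarts, tracks it and binds its restart request.
; Tick advances BP_GameState from Lobby through Tutorial to Battle, ending when any pawn's HP runs out.
; Restart resets Lobby and hand HP, while GameEnded requests Victory/Defeat widgets, created only on the Remote authority branch.
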(event `self.ReceiveBeginPlay`
  ;[1 1 1] Begin and Get All PlayerStart
  (`/Engine/EditorBlueprintResources/ActorMacros.Switch Has Authority`
    (:`Authority`
      (bind _outactors (`GameplayStatics.GetAllActorsOfClass` "/Script/Engine.PlayerStart"))
      (set `self.PlayerStartArray` _outactors))))

(event `self.K2_PostLogin`
  (params (NewPlayer :type "PlayerController Object Reference"))
  (bind _playersingame (`self.PlayersIngame`))
  ;[1 1 1] When a player joins game
  (`/Engine/EditorBlueprintResources/ActorMacros.Switch Has Authority`
    (:`Authority`
      (set `self.NewPlayer` NewPlayer)
      (bind _outactors (`GameplayStatics.GetAllActorsOfClass` "/Script/Engine.PlayerStart"))
      (switch `int` _playersingame
        (:`Default`
          _)
        (:`0`
          _))
      (set `self.PawnClass` "/Game/Blueprints/Characters/BP_Hands.BP_Hands_C")
      (bind _returnvalue (`|SpawnActorFromClass` (`self.PawnClass`) (`self.GetTransform` (`|GetArrayItem` _outactors (`KismetMathLibrary.Min` _playersingame 1))) "AdjustIfPossibleButAlwaysSpawn" "OverrideRootScale" null null))
      (`Controller.Possess` (`self.NewPlayer`) _returnvalue)
      (`/Engine/EditorBlueprintResources/StandardMacros.IncrementInt` (`self.PlayersIngame`)
        (:`  `
          (`KismetArrayLibrary.Array_AddUnique` (`self.PlayerPawns`) _returnvalue)
          (bind _asbp_hands (cast `/Game/Blueprints/Characters/BP_Hands` _returnvalue))
          (add `/Game/Blueprints/Characters/BP_Hands.GameRestartRequested` _asbp_hands (delegate `OnGameRestartRequested`))
          (`self.PlayerConnected`))))))

(event `self.ReceiveTick`
  (params (DeltaSeconds :type "Float (single-precision)"))
  (bind _asbp_game_state (cast `/Game/Blueprints/Gameplay/BP_GameState` (`GameplayStatics.GetGameState`)))
  (switch `/Game/Blueprints/Gameplay/EArenaGameStates` (`/Game/Blueprints/Gameplay/BP_GameState.GameState` _asbp_game_state)
    (:`NewEnumerator3`
      (set `/Game/Blueprints/Gameplay/BP_GameState.GameState` "NewEnumerator0" _asbp_game_state))
    (:`NewEnumerator0`
      (set `/Game/Blueprints/Gameplay/BP_GameState.GameState` "NewEnumerator1" _asbp_game_state))
    (:`NewEnumerator1`
      (for _array_element (`self.PlayerPawns`)
        (bind _asbp_hands (cast `/Game/Blueprints/Characters/BP_Hands` _array_element)
          (:`then`
            (if (<= (`/Game/Blueprints/Characters/BP_Hands.HitPoints` _asbp_hands) 0.0)
              (set `/Game/Blueprints/Gameplay/BP_GameState.GameState` "NewEnumerator2" _asbp_game_state :!label _label)
              (`KismetSystemLibrary.Delay` 0.5)
              (`self.OnGameEnded`)
              (break)))
          (:`CastFailed`
            (bind _asbp_arena_character (cast `/Game/Blueprints/Characters/BP_ArenaCharacter` _array_element))
            (if (<= (`/Game/Blueprints/Characters/BP_ArenaCharacter.HitPoints` _asbp_arena_character) 0.0)
              (goto _label))))))))

(event `OnGameRestartRequested`
  ;[1 1 1] Restart Level
  (bind _asbp_game_state (cast `/Game/Blueprints/Gameplay/BP_GameState` (`GameplayStatics.GetGameState`)))
  (set `/Game/Blueprints/Gameplay/BP_GameState.GameState` "NewEnumerator3" _asbp_game_state)
  (for _array_element (`self.PlayerPawns`)
    (bind _asbp_hands (cast `/Game/Blueprints/Characters/BP_Hands` _array_element))
    (set `/Game/Blueprints/Characters/BP_Hands.HitPoints` (`self.MaxHitPoints`) _asbp_hands)
    (`/Game/Blueprints/Characters/BP_Hands.CreateHpActors` _asbp_hands)))

(event `GameEnded`
  ;[1 1 1] End of game
  (for (_array_element _array_index) (`self.PlayerPawns`)
    (bind _asbp_hands (cast `/Game/Blueprints/Characters/BP_Hands` _array_element)
      (:`then`
        (`self.CreateHudWidget` _array_index (<= (`/Game/Blueprints/Characters/BP_Hands.HitPoints` _asbp_hands) 0.0)))
      (:`CastFailed`
        (bind _asbp_arena_character (cast `/Game/Blueprints/Characters/BP_ArenaCharacter` _array_element))
        (`self.CreateHudWidget` _array_index (<= (`/Game/Blueprints/Characters/BP_ArenaCharacter.HitPoints` _asbp_arena_character) 0.0))))))

(fn `CreateHudWidget`
  (params (`Player Index` :type Integer) (HasLost :type Boolean))
  (bind _returnvalue (`GameplayStatics.GetPlayerController` `Player Index`))
  (`/Engine/EditorBlueprintResources/ActorMacros.Switch Has Authority`
    (:`Remote`
      (if HasLost
        (bind _returnvalue_2 (`|CreateWidget` "/Game/Blueprints/Widgets/Defeat.Defeat_C" _returnvalue))
        (`UserWidget.AddToViewport` _returnvalue_2 0)
        (`UserWidget.AddToViewport` (stale _returnvalue_3) 0)
        (else
          (bind _returnvalue_3 (`|CreateWidget` "/Game/Blueprints/Widgets/Victory.Victory_C" _returnvalue)))))))

(fn `OnRep_GameRestartConfirmed`)

(fn `ReadyToStartMatch`
  (returns (ReturnValue :type Boolean))
  (bind _returnvalue (`self.GetNumPlayers`))
  (return (== _returnvalue (`self.MaxPlayerCount`))))

(fn `UserConstructionScript`)