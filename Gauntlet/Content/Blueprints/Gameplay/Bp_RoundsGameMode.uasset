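; Game mode for a two-player, round-based spell duel that colors players and platforms, then starts a countdown once both join.
; Tick switches Countdown to Battle, and a player death clears spells, awards the round and starts the next or ends on majority or round limit.
; Spawned round-point actors at each player start show round winners by color.
; A sudden death event removes scoreboard and walls and drops players to one hit point.
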(event `self.ReceiveBeginPlay`
  (`parent.ReceiveBeginPlay`)
  (set `/Game/Blueprints/Gameplay/BP_GameState.CurrentRound` 1.0 (`self.GameStateRef`))
  (`self.SpawnScoreboard`))

(event `self.ReceiveTick`
  (params (DeltaSeconds :type "Float (single-precision)"))
  (bind _gamestateref (`self.GameStateRef`))
  (bind _gamestateref_2 (`self.GameStateRef`))
  (switch `/Game/Blueprints/Gameplay/EArenaGameStates` (`/Game/Blueprints/Gameplay/BP_GameState.GameState` _gamestateref)
    (:`NewEnumerator4`
      (if (`/Game/Blueprints/Gameplay/BP_GameState.CountdownEnded` _gamestateref)
        (set `/Game/Blueprints/Gameplay/BP_GameState.GameState` "NewEnumerator1" _gamestateref)
        (for _array_element (`self.PlayerPawns`)
          (bind _asbp_hands (cast `/Game/Blueprints/Characters/BP_Hands` _array_element))
          (set `/Game/Blueprints/Characters/BP_Hands.Invincible` false _asbp_hands))))
    (:`NewEnumerator1`
      (for _array_element_2 (`self.PlayerPawns`)
        (bind _asbp_hands_2 (cast `/Game/Blueprints/Characters/BP_Hands` _array_element_2))
        (if (<= (`/Game/Blueprints/Characters/BP_Hands.HitPoints` _asbp_hands_2) 0.0)
          (`self.ClearSpells`)
          (`self.AssignPoints`)
          (for _array_element_3 (`self.PlayerPawns`)
            (bind _asbp_arena_player_state (cast `/Game/Blueprints/Gameplay/BP_ArenaPlayerState` (`Pawn.PlayerState` _array_element_3)))
            (bind _roundwins (`/Game/Blueprints/Gameplay/BP_ArenaPlayerState.RoundWins` _asbp_arena_player_state))
            (if (> _roundwins (`self.MaxPointsScored`))
              (set `self.MaxPointsScored` _roundwins)))
          (if (or (>= (`/Game/Blueprints/Gameplay/BP_GameState.CurrentRound` (`self.GameStateRef`)) (`self.MaxRounds`)) (>= (`self.MaxPointsScored`) (`KismetMathLibrary.Conv_IntToDouble` (`KismetMathLibrary.FCeil` (/ (`self.MaxRounds`) 2.0)))))
            (`self.EndGame`)
            (break)
            (else
              (bind _result (`/Engine/EditorBlueprintResources/StandardMacros.IncrementFloat` (`/Game/Blueprints/Gameplay/BP_GameState.CurrentRound` _gamestateref_2))
                (:`  `
                  (set `/Game/Blueprints/Gameplay/BP_GameState.CurrentRound` _result _gamestateref_2)
                  (`/Game/Blueprints/Gameplay/BP_GameState.StartCountdown` _gamestateref_2 3.0)
                  (set `/Game/Blueprints/Gameplay/BP_GameState.GameState` "NewEnumerator4" (`self.GameStateRef`))
                  (`self.StartNewRound`)
                  (break))))))))))

(event `self.K2_PostLogin`
  (params (NewPlayer :type "PlayerController Object Reference"))
  (bind _gamestateref (`self.GameStateRef`))
  (bind _player1color (`self.Player1Color`))
  (bind _player2color (`self.Player2Color`))
  (bind _playerpawns (`self.PlayerPawns`))
  (`parent.K2_PostLogin` NewPlayer)
  (if (== (`KismetArrayLibrary.Array_Length` _playerpawns) 2)
    (for _array_element _playerpawns
      (bind _asbp_arena_player_state (cast `/Game/Blueprints/Gameplay/BP_ArenaPlayerState` (`Pawn.PlayerState` _array_element)))
      (`/Game/Blueprints/Gameplay/BP_ArenaPlayerState.SetScore` _asbp_arena_player_state 0.0))
    ;[1 1 1] Set character color
    (`/Engine/EditorBlueprintResources/ActorMacros.Switch Has Authority`
      (:`Authority`
        (bind _asbp_hands (cast `/Game/Blueprints/Characters/BP_Hands` (`|GetArrayItem` (`self.PlayerPawns`))))
        (set `/Game/Blueprints/Characters/BP_Hands.PlayerColor` _player1color _asbp_hands)
        (set `/Game/Blueprints/Characters/BP_Hands.LeftHandColor` _player1color _asbp_hands)
        (set `/Game/Blueprints/Characters/BP_Hands.RightHandColor` _player1color _asbp_hands)
        (bind _asbp_hands_2 (cast `/Game/Blueprints/Characters/BP_Hands` (`|GetArrayItem` (`self.PlayerPawns`) 1)))
        (set `/Game/Blueprints/Characters/BP_Hands.PlayerColor` _player2color _asbp_hands_2)
        (set `/Game/Blueprints/Characters/BP_Hands.LeftHandColor` _player2color _asbp_hands_2)
        (set `/Game/Blueprints/Characters/BP_Hands.RightHandColor` _player2color _asbp_hands_2)
        (if (== (`self.PlayersIngame`) 2)
          (`self.ColorPlatforms`)
          ;[1 1 1] Start countdown when both players joined
          (`KismetSystemLibrary.Delay` 1.0)
          (for _array_element_2 (`self.PlayerPawns`)
            (bind _asbp_hands_3 (cast `/Game/Blueprints/Characters/BP_Hands` _array_element_2))
            (`/Game/Blueprints/Characters/BP_Hands.CallShowColor` _asbp_hands_3))
          (`KismetSystemLibrary.Delay` 3.0)
          (set `/Game/Blueprints/Gameplay/BP_GameState.GameState` "NewEnumerator4" _gamestateref)
          (`/Game/Blueprints/Gameplay/BP_GameState.StartCountdown` _gamestateref 3.0))))))

(event `OnSuddenDeath`
  (set `self.MaxHitPoints` 1.0)
  (for _array_element (`self.PlayerPawns`)
    (bind _asbp_hands (cast `/Game/Blueprints/Characters/BP_Hands` _array_element))
    (bind _asbp_arena_player_state (cast `/Game/Blueprints/Gameplay/BP_ArenaPlayerState` (`Pawn.PlayerState` _asbp_hands)))
    (`/Game/Blueprints/Gameplay/BP_ArenaPlayerState.SetScore` _asbp_arena_player_state 1.0)
    (set `/Game/Blueprints/Characters/BP_Hands.HitPoints` 1.0 _asbp_hands))
  (bind _outactors (`GameplayStatics.GetAllActorsOfClass` "/Game/Blueprints/BP_RoundPoint.BP_RoundPoint_C"))
  (for _array_element_2 _outactors
    (`self.K2_DestroyActor` _array_element_2))
  (bind _outactors_2 (`GameplayStatics.GetAllActorsOfClass` "/Game/Blueprints/Gameplay/BP_Wall.BP_Wall_C"))
  (for _array_element_3 _outactors_2
    (`self.K2_DestroyActor` _array_element_3))
  (`self.StartSuddenDeath`))

(fn `AssignPoints`
  (locals (FirstIndex :type Integer :default 0) (SecondIndex :type Integer :default 0) (ScoringPlayerIndex :type Integer))
  (`|ExecutionSequence`
    (:`then_0`
      (for (_array_element _array_index) (`self.PlayerPawns`)
        (bind _asbp_hands (cast `/Game/Blueprints/Characters/BP_Hands` _array_element))
        (if (> (`/Game/Blueprints/Characters/BP_Hands.HitPoints` _asbp_hands) 0.0)
          (bind _asbp_arena_player_state (cast `/Game/Blueprints/Gameplay/BP_ArenaPlayerState` (`Pawn.PlayerState` _asbp_hands)))
          (`/Game/Blueprints/Gameplay/BP_ArenaPlayerState.SetScore` _asbp_arena_player_state (+ (`/Game/Blueprints/Gameplay/BP_ArenaPlayerState.RoundWins` _asbp_arena_player_state) 1.0))
          (set `local.ScoringPlayerIndex` _array_index)))
      (`|ExecutionSequence`
        (:`then_0`
          (bind _output_get (set `local.FirstIndex` (- (`KismetMathLibrary.FTrunc` (`/Game/Blueprints/Gameplay/BP_GameState.CurrentRound` (`self.GameStateRef`))) 1)))
          (set `local.SecondIndex` (+ _output_get (`KismetMathLibrary.FTrunc` (`self.MaxRounds`))))
          (bind _asbp_hands_2 (cast `/Game/Blueprints/Characters/BP_Hands` (`|GetArrayItem` (`self.PlayerPawns`) (`local.ScoringPlayerIndex`))))
          (bind _playercolor (`/Game/Blueprints/Characters/BP_Hands.PlayerColor` _asbp_hands_2))
          (set `/Game/Blueprints/BP_RoundPoint.ScoringColor` _playercolor (`|GetArrayItem` (`self.ScoreObjects`) (`local.FirstIndex`)))
          (set `/Game/Blueprints/BP_RoundPoint.ScoringColor` _playercolor (`|GetArrayItem` (`self.ScoreObjects`) (`local.SecondIndex`))))
        (:`then_1`
          (for _array_element_2 (`self.PlayerPawns`)
            (bind _asbp_hands_3 (cast `/Game/Blueprints/Characters/BP_Hands` _array_element_2))
            (bind _createdwidget (`/Game/Blueprints/Characters/BP_Hands.ShowWidget` _asbp_hands_3 "/Game/Blueprints/Widgets/BP_RoundWinner.BP_RoundWinner_C"))
            (bind _asbp_round_winner (cast `/Game/Blueprints/Widgets/BP_RoundWinner` _createdwidget))
            (`/Game/Blueprints/Widgets/BP_RoundWinner.Initialize` _asbp_round_winner _playercolor)))))))

(fn `ClearSpells`
  (`|ExecutionSequence`
    (:`then_0`
      ;[1 1 1] Destroy Fireballs
      (bind _outactors (`GameplayStatics.GetAllActorsOfClass` "/Game/Blueprints/GestureSpells/Spells/BP_Fireball.BP_Fireball_C"))
      (for _array_element _outactors
        (`/Game/Blueprints/GestureSpells/Spells/BP_Fireball.OnDestroy` _array_element _array_element)))
    (:`then_1`
      ;[1 1 1] Destroy Shields
      (bind _outactors_2 (`GameplayStatics.GetAllActorsOfClass` "/Game/Blueprints/GestureSpells/Spells/BP_Shield.BP_Shield_C"))
      (for _array_element_2 _outactors_2
        (`/Game/Blueprints/GestureSpells/Hand.SetShieldUp` (`/Game/Blueprints/GestureSpells/Spells/BP_Shield.Hand` _array_element_2) false)))
    (:`then_2`
      ;[1 1 1] Reset hands properties
      (for _array_element_3 (`self.PlayerPawns`)
        (bind _asbp_hands (cast `/Game/Blueprints/Characters/BP_Hands` _array_element_3))
        (`/Game/Blueprints/Characters/BP_Hands.ResetHands` _asbp_hands)))))

(fn `ColorPlatforms`
  (bind _outactors (`GameplayStatics.GetAllActorsOfClass` "/Game/Blueprints/Gameplay/BP_Platform.BP_Platform_C"))
  (for _array_element _outactors
    (for _array_element_2 (`self.PlayerPawns`)
      (if (<= (`self.GetDistanceTo` _array_element_2 _array_element) 200.0)
        (bind _asbp_hands (cast `/Game/Blueprints/Characters/BP_Hands` _array_element_2))
        (set `/Game/Blueprints/Gameplay/BP_Platform.Color` (`/Game/Blueprints/Characters/BP_Hands.PlayerColor` _asbp_hands) _array_element)))))

(fn `EndAudio`
  (bind _outactors (`GameplayStatics.GetAllActorsOfClass` "/Game/Blueprints/Characters/BP_Audio_Arena.BP_Audio_Arena_C"))
  (for _array_element _outactors
    (`/Game/Blueprints/Characters/BP_Audio_Arena.StopAudio` _array_element))
  (return))

(fn `EndGame`
  (locals (Winner :type "Pawn Object Reference") (MaxScore :type "Float (double-precision)"))
  (bind _winner (`local.Winner`))
  (bind _playerpawns (`self.PlayerPawns`))
  (set `/Game/Blueprints/Gameplay/BP_GameState.GameState` "NewEnumerator2" (`self.GameStateRef`))
  (for _array_element (`self.PlayerPawns`)
    (bind _asbp_arena_player_state (cast `/Game/Blueprints/Gameplay/BP_ArenaPlayerState` (`Pawn.PlayerState` _array_element)))
    (if (>= (`/Game/Blueprints/Gameplay/BP_ArenaPlayerState.RoundWins` _asbp_arena_player_state) (`self.MaxPointsScored`))
      (set `local.Winner` _array_element)
      (break)))
  (for _array_element_2 (`self.PlayerPawns`)
    (bind _asbp_hands (cast `/Game/Blueprints/Characters/BP_Hands` _array_element_2))
    (`/Engine/EditorBlueprintResources/StandardMacros.IsValid` _winner
      (:`Is Valid`
        (`/Game/Blueprints/Characters/BP_Hands.GameEnded` _asbp_hands _winner)
        (`self.ClearSpells`))
      (:`Is Not Valid`
        (for _array_element_3 _playerpawns
          (bind _asbp_arena_player_state_2 (cast `/Game/Blueprints/Gameplay/BP_ArenaPlayerState` (`Pawn.PlayerState` _array_element_3)))
          (bind _roundwins (`/Game/Blueprints/Gameplay/BP_ArenaPlayerState.RoundWins` _asbp_arena_player_state_2))
          (if (> _roundwins (`local.MaxScore`))
            (set `local.Winner` _array_element_3)
            (set `local.MaxScore` _roundwins)))
        (for _array_element_4 _playerpawns
          (bind _asbp_hands_2 (cast `/Game/Blueprints/Characters/BP_Hands` _array_element_4))
          (`/Game/Blueprints/Characters/BP_Hands.GameEnded` _asbp_hands_2 (`local.Winner`))))))
  (`self.OnGameEnded` (`local.Winner`))
  (`self.EndAudio`)
  (return))

(fn `SpawnScoreboard`
  (bind _returnvalue (`KismetMathLibrary.FTrunc` (`self.MaxRounds`)))
  (for _array_element (`self.PlayerStartArray`)
    (for _index (range 1 (+ (`KismetMathLibrary.FTrunc` (`self.MaxRounds`)) 1))
      (bind _returnvalue_2 (`|SpawnActorFromClass` "/Game/Blueprints/BP_RoundPoint.BP_RoundPoint_C" (`KismetMathLibrary.MakeTransform` (+ (.location (`self.GetTransform` _array_element)) (0.0 0.0 150.0) (* (* (`self.GetActorRightVector` _array_element) (`KismetMathLibrary.MakeVector` (+ (* (/ (* (`self.MaxRounds`) 75.0) 2.0) -1.0) (* (- (`KismetMathLibrary.Conv_IntToDouble` _index) 1.0) 75.0) 37.0))) -1.0) (* (`self.GetActorForwardVector` _array_element) -100.0)) (.rotation (`self.GetTransform` _array_element)) (.scale (`self.GetTransform` _array_element))) "Undefined" "OverrideRootScale" null null))
      (bind _returnvalue_3 (`KismetArrayLibrary.Array_Add` (`self.ScoreObjects`) _returnvalue_2))
      (bind _result (`/Engine/EditorBlueprintResources/StandardMacros.IncrementInt` _returnvalue_3)
        (:`  `
          (if (<= _result _returnvalue)
            (set `/Game/Blueprints/BP_RoundPoint.AssociatedNumber` _result _returnvalue_2)
            (else
              (set `/Game/Blueprints/BP_RoundPoint.AssociatedNumber` (- _result _returnvalue) _returnvalue_2))))))))

(fn `StartNewRound`
  (for _array_element (`self.PlayerPawns`)
    (bind _asbp_hands (cast `/Game/Blueprints/Characters/BP_Hands` _array_element))
    (set `/Game/Blueprints/Characters/BP_Hands.HitPoints` (`self.MaxHitPoints`) _asbp_hands))
  (bind _outactors (`GameplayStatics.GetAllActorsOfClass` "/Game/Blueprints/BP_HealthPoint.BP_HealthPoint_C"))
  (for _array_element_2 _outactors
    (`self.K2_DestroyActor` _array_element_2))
  (for _array_element_3 (`self.PlayerPawns`)
    (bind _asbp_hands_2 (cast `/Game/Blueprints/Characters/BP_Hands` _array_element_3))
    (`/Game/Blueprints/Characters/BP_Hands.CreateHpActors` _asbp_hands_2)
    (set `/Game/Blueprints/Characters/BP_Hands.Invincible` true _asbp_hands_2))
  (bind _outactors_2 (`GameplayStatics.GetAllActorsOfClass` "/Game/Blueprints/Characters/BP_Audio_Arena.BP_Audio_Arena_C"))
  (for _array_element_4 _outactors_2
    (`/Game/Blueprints/Characters/BP_Audio_Arena.OnRoundChange` _array_element_4)))

(fn `StartSuddenDeath`
  (for _array_element (`self.PlayerPawns`)
    (bind _asbp_hands (cast `/Game/Blueprints/Characters/BP_Hands` _array_element))
    (set `/Game/Blueprints/Characters/BP_Hands.HitPoints` (`self.MaxHitPoints`) _asbp_hands))
  (bind _outactors (`GameplayStatics.GetAllActorsOfClass` "/Game/Blueprints/BP_HealthPoint.BP_HealthPoint_C"))
  (for _array_element_2 _outactors
    (`self.K2_DestroyActor` _array_element_2))
  (for _array_element_3 (`self.PlayerPawns`)
    (bind _asbp_hands_2 (cast `/Game/Blueprints/Characters/BP_Hands` _array_element_3))
    (`/Game/Blueprints/Characters/BP_Hands.CreateHpActors` _asbp_hands_2)
    (set `/Game/Blueprints/Characters/BP_Hands.Invincible` false _asbp_hands_2)
    (`/Game/Blueprints/Characters/BP_Hands.CallShowSuddenDeath` _asbp_hands_2)))

(fn `UserConstructionScript`
  (`parent.UserConstructionScript`))