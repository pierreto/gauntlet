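; BP_AnimTester is a test Blueprint that replays saved two-hand gesture recordings in front of the camera.
; The PlayGesture input toggles playback, loading frames from a RecordingSaveGame slot.
; Tick consumes timed frames, setting hand mesh transforms relative to the camera's starting location and yaw, plus pose snapshots.
; It also sets hand ticking from RecognizeGesture and provides hand-center, distance and fireball-scale helpers.
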(event `self.ReceiveBeginPlay`
  ;[1 1 1] Save initial hand pose
  (`KismetSystemLibrary.PrintString` (`KismetStringLibrary.Concat_StrStr` "THIS: " (`KismetSystemLibrary.GetDisplayName` (`SkeletalMeshComponent.GetAnimInstance` (`self.BodySM`)))))
  (`SkeletalMeshComponent.SnapshotPose` (`self.SkeletalMeshL`) (`self.InitialLeftPose`))
  (`SkeletalMeshComponent.SnapshotPose` (`self.SkeletalMeshR`) (`self.InitialRightPose`))
  (set `/Game/Blueprints/GestureSpells/Hand.ShouldTick` (`self.RecognizeGesture`) (`self.LeftHand`))
  (set `/Game/Blueprints/GestureSpells/Hand.ShouldTick` (`self.RecognizeGesture`) (`self.RightHand`)))

(event `self.ReceiveTick`
  (params (DeltaSeconds :type "Float (single-precision)"))
  ;[1 1 1] Play recording
  (`|ExecutionSequence`
    (:`then_0`
      (if (`self.IsPlayingRecording`)
        (`self.PlayRecording` (`self.Recordings`) DeltaSeconds)
        (if (or (<= (`KismetArrayLibrary.Array_Length` (`self.Recordings`)) 0) (>= (`self.CurrentReplayTime`) (`self.EndTime`)))
          (set `self.IsPlayingRecording` false)
          (`KismetSystemLibrary.PrintString` "Finished playing"))))))

(event `InputAction|PlayGesture`
  (params (Key :type "Key Structure"))
  ;[1 1 1] Load gesture recording and start playing
  (:`Released`
    (if (`self.IsPlayingRecording`)
      (set `self.IsPlayingRecording` false)
      (else
        (bind (_recordings _success) (`self.LoadRecording` (`self.SaveSlot`)))
        (if _success
          (`self.Play` _recordings)
          (else
            (`KismetSystemLibrary.PrintString` "Failed to load recording!" true true (struct :`R` 1.0 :`A` 1.0))))))))

(event `InputAction|Exit`
  (params (Key :type "Key Structure"))
  ;[1 1 1] Quit
  (:`Pressed`
    (`KismetSystemLibrary.QuitGame` null "Quit")))

(fn `GetFireballScale`
  (returns (Scale :type "Vector Structure"))
  (bind _returnvalue (/ (`KismetMathLibrary.FClamp` (`self.GetHandsDistance`) 10.0 100.0) 100.0))
  (return (`KismetMathLibrary.MakeVector` _returnvalue _returnvalue _returnvalue)))

(fn `GetHandsCenter`
  (returns (Center :type "Vector Structure"))
  (return (/ (+ (`/Game/Blueprints/GestureSpells/Hand.GetHandCenter` (`self.RightHand`)) (`/Game/Blueprints/GestureSpells/Hand.GetHandCenter` (`self.LeftHand`))) 2)))

(fn `GetHandsDistance`
  (returns (Distance :type "Float (double-precision)"))
  (return (`KismetMathLibrary.VSize` (- (`SceneComponent.K2_GetComponentLocation` (`self.SkeletalMeshL`)) (`SceneComponent.K2_GetComponentLocation` (`self.SkeletalMeshR`))))))

(fn `GetWorldTransform`
  (params (Transform :type "Transform Structure"))
  (returns (WorldTransform :type "Transform Structure"))
  (bind _initialcameratransform (`self.InitialCameraTransform`))
  ;[1 1 1] Replay in front of camera
  (return (`KismetMathLibrary.MakeTransform` (+ (`KismetMathLibrary.RotateAngleAxis` (.location Transform) (.yaw (.rotation _initialcameratransform)) (0.0 0.0 1.0)) (.location _initialcameratransform)) (`KismetMathLibrary.MakeRotator` (.roll (.rotation Transform)) (.pitch (.rotation Transform)) (+ (.yaw (.rotation Transform)) (.yaw (.rotation _initialcameratransform)))) (.scale Transform))))

(fn `LoadRecording`
  (params (SaveSlot :type String))
  (returns (Recordings :type "Array of /Game/Blueprints/Dev/Record/GestureRecording Structure") (Success :type Boolean))
  (locals (Loaded :type Boolean) (_recordings :type "Array of /Game/Blueprints/Dev/Record/GestureRecording Structure"))
  (`KismetSystemLibrary.PrintString` "Loading...")
  (`GameplayStatics.CreateSaveGameObject` "/Game/Blueprints/Dev/Record/RecordingSaveGame.RecordingSaveGame_C")
  (bind _returnvalue (`GameplayStatics.LoadGameFromSlot` SaveSlot))
  (if (`KismetSystemLibrary.IsValid` _returnvalue)
    (bind _asrecording_save_game (cast `/Game/Blueprints/Dev/Record/RecordingSaveGame` _returnvalue))
    (bind _recordings (`/Game/Blueprints/Dev/Record/RecordingSaveGame.Recordings` _asrecording_save_game))
    (set `local._recordings` _recordings)
    (`KismetSystemLibrary.PrintString` (`KismetStringLibrary.Concat_StrStr` "Loaded : " (`KismetStringLibrary.Conv_IntToString` (`KismetArrayLibrary.Array_Length` _recordings)) " recordings!"))
    (set `local.Loaded` true))
  (return (`local._recordings`) (`local.Loaded`)))

(fn `Play`
  (params (Recordings :type "Array of /Game/Blueprints/Dev/Record/GestureRecording Structure"))
  (set `self.IsPlayingRecording` true)
  (set `self.Recordings` Recordings)
  (set `self.CurrentReplayTime` 0.0)
  (set `self.InitialCameraTransform` (`SceneComponent.K2_GetComponentToWorld` (`self.Camera`)))
  (`KismetSystemLibrary.PrintString` "Start playing"))

(fn `PlayRecording`
  (params (Recordings :type "Array of /Game/Blueprints/Dev/Record/GestureRecording Structure (by ref)") (DeltaTime :type "Float (double-precision)"))
  (bind (_leftpose _rightpose _lefttransform _righttransform _recordtime) (break `/Game/Blueprints/Dev/Record/GestureRecording` (`|GetArrayItem` Recordings)))
  (bind _output_get (set `self.CurrentReplayTime` (+ DeltaTime (`self.CurrentReplayTime`))))
  (if (>= _output_get _recordtime)
    (bind _worldtransform (`self.GetWorldTransform` _lefttransform))
    (`SceneComponent.K2_SetWorldTransform` (`self.SkeletalMeshL`) _worldtransform false false)
    (bind _worldtransform_2 (`self.GetWorldTransform` _righttransform))
    (`SceneComponent.K2_SetWorldTransform` (`self.SkeletalMeshR`) _worldtransform_2 false false)
    (`KismetArrayLibrary.Array_Remove` Recordings)
    (set `self.CurrentLeftPose` _leftpose)
    (set `self.CurrentRightPose` _rightpose)))

(fn `ResetHands`
  (set `self.CurrentLeftPose` (`self.InitialLeftPose`))
  (set `self.CurrentRightPose` (`self.InitialRightPose`)))

(fn `Stop`
  (set `self.IsPlayingRecording` false)
  (set `self.CurrentReplayTime` 0.0))

(fn `UserConstructionScript`)