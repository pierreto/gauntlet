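; Networked VR player pawn for a wizard duel, with a wizard body that follows the replicated headset camera.
; On the owning client, Tick follows the game state, running both hands' gesture detection in Tutorial and Battle and showing a camera-attached countdown between.
; Damage removes authority-spawned health-point actors, and game end shows a camera-attached victory or defeat widget, with restart and tutorial inputs.
; Two-handed fireball helpers exist, but their handler is disconnected.
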(event `ShowEndGameClient`
  ;[1 1 1] Show end game client
  (`self.CreateEndGameWidget` (< (`self.HitPoints`) 1.0)))

(event `self.ReceiveBeginPlay`
  (bind _replicatedvrcamera (`self.ReplicatedVRCamera`))
  ;[1 1 1] Set Character Start Attributes
  (`|ExecutionSequence`
    (:`then_1`
      (bind _asbp_game_state (cast `/Game/Blueprints/Gameplay/BP_GameState` (`GameplayStatics.GetGameState`)))
      (set `self.GameStateRef` _asbp_game_state)
      (`HeadMountedDisplayFunctionLibrary.SetTrackingOrigin` "Floor")
      (set `/Game/Blueprints/GestureSpells/Hand.VRCameraRef` _replicatedvrcamera (`self.HandR`))
      (set `/Game/Blueprints/GestureSpells/Hand.VRCameraRef` _replicatedvrcamera (`self.HandL`))
      (`/Engine/EditorBlueprintResources/ActorMacros.Switch Has Authority`
        (:`Authority`
          (`self.CreateHpActors`))))))

(event `GameEnded`
  ;[1 1 1] Set Character Start Attributes
  (`self.ShowEndGameClient`))

(event `InputAction|RestartLevel`
  (params (Key :type "Key Structure"))
  ;[1 1 1] Restart Level
  (:`Pressed`
    (bind _asbp_game_state (cast `/Game/Blueprints/Gameplay/BP_GameState` (`GameplayStatics.GetGameState`)))
    (switch `/Game/Blueprints/Gameplay/EArenaGameStates` (`/Game/Blueprints/Gameplay/BP_GameState.GameState` _asbp_game_state)
      (:`NewEnumerator2`
        (`/Engine/EditorBlueprintResources/ActorMacros.Switch Has Authority`
          (:`Authority`
            (`self.GameRestartRequested`)
            (`self.RestartClient`)))))))

(event `self.ReceiveAnyDamage`
  (params (Damage :type "Float (single-precision)") (DamageType :type "DamageType Object Reference") (InstigatedBy :type "Controller Object Reference") (DamageCauser :type "Actor Object Reference"))
  ;[1 1 1] Damage
  (`self.IndicateHit`)
  (if (not (`self.Invincible`))
    (set `self.HitPoints` (- (`self.HitPoints`) Damage))
    (`self.DestroyHpActor`)
    (`self.ShowHUDHitEffect`)))

(event `RestartClient`
  ;[1 1 1] Restart Level
  (`self.DestroyWidget`))

(event `InputAction|Exit`
  (params (Key :type "Key Structure"))
  ;[1 1 1] Quit
  (:`Pressed`
    (`KismetSystemLibrary.QuitGame` null "Quit")))

(event `InputAction|BackToTutorial`
  (params (Key :type "Key Structure"))
  (:`Pressed`
    (bind _asbp_game_state (cast `/Game/Blueprints/Gameplay/BP_GameState` (`GameplayStatics.GetGameState`)))
    (switch `/Game/Blueprints/Gameplay/EArenaGameStates` (`/Game/Blueprints/Gameplay/BP_GameState.GameState` _asbp_game_state)
      (:`NewEnumerator2`
        (`self.OpenTutorial`)))))

(event `OpenTutorial`
  (`GameplayStatics.OpenLevel` "ArenaTutorial"))

(event `Key|H`
  (params (Key :type "Key Structure"))
  (:`Pressed`
    (`GameplayStatics.ApplyDamage` self 1.0)))

(event `self.ReceiveTick`
  (params (DeltaSeconds :type "Float (single-precision)"))
  ;[1 1 1] Move Wizard
  (`self.UpdateWizardTransform`)
  (if (`self.HasOwnership`)
    (`|ExecutionSequence`
      (:`then_1`
        (switch `/Game/Blueprints/Gameplay/EArenaGameStates` (`/Game/Blueprints/Gameplay/BP_GameState.GameState` (`self.GameStateRef`))
          (:`NewEnumerator3`
            ;[1 1 1] Detect gestures
            (`/Game/Blueprints/GestureSpells/Hand.HandleRightGesture` (`self.HandR`) :!label _label)
            (`/Game/Blueprints/GestureSpells/Hand.HandleLeftGesture` (`self.HandL`)))
          (:`NewEnumerator4`
            ;[1 1 1] Show countdown
            (`/Engine/EditorBlueprintResources/StandardMacros.IsValid` (`self.CountdownActor`)
              (:`Is Valid`
                (`self.ShowCountdown`))
              (:`Is Not Valid`
                (`self.StartCountdown`))))
          (:`NewEnumerator1`
            ;[1 1 1] Hide countdown
            (`/Engine/EditorBlueprintResources/StandardMacros.IsValid` (`self.CountdownActor`)
              (:`Is Valid`
                (`self.K2_DestroyActor` (`self.CountdownActor`))
                (goto _label))
              (:`Is Not Valid`
                (goto _label)))))))))

(event `Key|S`
  (params (Key :type "Key Structure"))
  ;[1 1 1] Skip tutorial
  (:`Released`
    (bind _outactors (`GameplayStatics.GetAllActorsOfClass` "/Game/Blueprints/Characters/BP_Tutorial.BP_Tutorial_C"))
    (set `/Game/Blueprints/Characters/BP_Tutorial.TutorialState` "NewEnumerator6" (`|GetArrayItem` _outactors))))

(event `ShowHUDHitEffect`
  (cast `/Game/Blueprints/Widgets/HitEffect` (`WidgetComponent.GetUserWidgetObject` (`self.HitEffect`))))

(fn `CreateEndGameWidget`
  (params (HasLost :type Boolean))
  (if HasLost
    (`self.ShowWidget` "/Game/Blueprints/Widgets/BP_Defeat.BP_Defeat_C")
    (else
      (`self.ShowWidget` "/Game/Blueprints/Widgets/BP_Victory.BP_Victory_C"))))

(fn `CreateHpActors`
  (bind _output_get (set `self.HitPoints` (`self.HitPoints`)))
  (bind _closestactor (`self.GetClosestActor` "/Script/Engine.PlayerStart"))
  (for _index (range 1 (+ (`KismetMathLibrary.FTrunc` _output_get) 1))
    (bind _returnvalue (`|SpawnActorFromClass` "/Game/Blueprints/BP_HealthPoint.BP_HealthPoint_C" (`self.DefaultTransform`) "AlwaysSpawn" "OverrideRootScale" null null))
    (bind _rootcomponent (`Actor.RootComponent` _closestactor))
    (bind _returnvalue_2 (`SceneComponent.GetUpVector` _rootcomponent))
    (bind (_returnvalue_x _returnvalue_y _returnvalue_z) (`KismetMathLibrary.BreakVector` (+ (`SceneComponent.K2_GetComponentLocation` _rootcomponent) (* _returnvalue_2 20) (* _returnvalue_2 (* _index (`self.HorizontalHpOffset`))) (* _returnvalue_2 (/ (* (+ _output_get 1.0) (`self.HorizontalHpOffset`)) -2.0)) (150.0 0.0 0.0))))
    (`self.K2_SetActorLocation` _returnvalue (`KismetMathLibrary.MakeVector` _returnvalue_x (* _returnvalue_y 0.7) _returnvalue_z) false false)
    (`KismetArrayLibrary.Array_Add` (`self.HpActors`) _returnvalue)))

(fn `DestroyHpActor`
  (bind _returnvalue (`KismetArrayLibrary.Array_Length` (`self.HpActors`)))
  (bind _returnvalue_2 (- _returnvalue 1))
  (if (> _returnvalue 0)
    (`/Game/Blueprints/BP_HealthPoint.OnHpRemoved` (`|GetArrayItem` (`self.HpActors`) _returnvalue_2))
    (`KismetArrayLibrary.Array_Remove` (`self.HpActors`) _returnvalue_2)))

(fn `DestroyWidget`
  (bind _outactors (`GameplayStatics.GetAllActorsOfClass` "/Game/Blueprints/Widgets/BP_Defeat.BP_Defeat_C"))
  (for _array_element _outactors
    (`self.K2_DetachFromActor` _array_element "KeepRelative" "KeepRelative" "KeepRelative")
    (`self.K2_DestroyActor` _array_element))
  (bind _outactors_2 (`GameplayStatics.GetAllActorsOfClass` "/Game/Blueprints/Widgets/BP_Victory.BP_Victory_C"))
  (for _array_element_2 _outactors_2
    (`self.K2_DetachFromActor` _array_element_2 "KeepRelative" "KeepRelative" "KeepRelative")
    (`self.K2_DestroyActor` _array_element_2)))

(fn `DetectShootFireball`
  (returns (Detected :type Boolean) (Direction :type "Vector Structure"))
  (bind _returnvalue (`SceneComponent.K2_GetComponentLocation` (`/Game/Blueprints/GestureSpells/Spells/BP_Fireball.Fire Ball` (`self.HeldFireball`))))
  (bind _returnvalue_2 (/ (+ (`/Game/Blueprints/GestureSpells/Hand.GetVelocity` (`self.HandR`)) (`/Game/Blueprints/GestureSpells/Hand.GetVelocity` (`self.HandL`))) 2))
  (bind _returnvalue_3 (`KismetMathLibrary.Normal` (- (`SceneComponent.K2_GetComponentLocation` (`/Game/Blueprints/GestureSpells/Spells/BP_Fireball.Fire Ball` (`self.HeldFireball`))) (- (`SceneComponent.K2_GetComponentLocation` (`self.ReplicatedVRCamera`)) (0.0 0.0 30.0)))))
  (bind _returnvalue_4 (`KismetMathLibrary.Dot_VectorVector` (`KismetMathLibrary.Normal` _returnvalue_2) (`KismetMathLibrary.Normal` (`KismetMathLibrary.Conv_Vector2DToVector` (- (`KismetMathLibrary.Conv_VectorToVector2D` (`SceneComponent.K2_GetComponentLocation` (`/Game/Blueprints/GestureSpells/Spells/BP_Fireball.Fire Ball` (`self.HeldFireball`)))) (`KismetMathLibrary.Conv_VectorToVector2D` (`SceneComponent.K2_GetComponentLocation` (`self.Character_Wizard_01`))))))))
  (bind _returnvalue_5 (and (> (`KismetMathLibrary.VSize` _returnvalue_2) 75.0) (> _returnvalue_4 0.5)))
  (`KismetSystemLibrary.DrawDebugArrow` _returnvalue (+ _returnvalue (* _returnvalue_3 50)) 1.0 (struct :`R` 1.0 :`A` 1.0) 0.0 1.0)
  (if _returnvalue_5
    (`KismetSystemLibrary.PrintString` (`KismetStringLibrary.Conv_DoubleToString` _returnvalue_4))
    (return _returnvalue_5 _returnvalue_3)))

(fn `GetClosestActor`
  (params (ObjectClass :type "Actor Class Reference"))
  (returns (ClosestActor :type "Actor Object Reference"))
  (locals (smallestDistance :type "Float (double-precision)" :default 999999.0) (closeActor :type "Actor Object Reference"))
  (bind _outactors (`GameplayStatics.GetAllActorsOfClass` ObjectClass))
  (for _array_element _outactors
    (bind _returnvalue (`self.GetDistanceTo` _array_element))
    (if (< _returnvalue (`local.smallestDistance`))
      (set `local.closeActor` _array_element)
      (set `local.smallestDistance` _returnvalue)))
  (return (`local.closeActor`)))

(fn `GetFireballScale`
  (returns (Scale :type "Vector Structure"))
  (bind _returnvalue (/ (`KismetMathLibrary.FClamp` (`self.GetHandsDistance`) 10.0 80.0) 100.0))
  (return (`KismetMathLibrary.MakeVector` _returnvalue _returnvalue _returnvalue)))

(fn `GetHandsCenter`
  (returns (Center :type "Vector Structure"))
  (return (/ (+ (`/Game/Blueprints/GestureSpells/Hand.GetHandCenter` (`self.HandR`)) (`/Game/Blueprints/GestureSpells/Hand.GetHandCenter` (`self.HandL`))) 2)))

(fn `GetHandsDistance`
  (returns (Distance :type "Float (double-precision)"))
  (return (`KismetMathLibrary.VSize` (- (`SceneComponent.K2_GetComponentLocation` (`self.SkeletalMeshL`)) (`SceneComponent.K2_GetComponentLocation` (`self.SkeletalMeshR`))))))

(fn `HandleDoubleHandGestures`
  (params (DeltaTime :type "Float (double-precision)"))
  (returns (Detected :type Boolean))
  (locals (_Detected :type Boolean :default true)))

(fn `HasOwnership`
  (returns (IsOwner :type Boolean))
  (return (== (`self.GetController`) (`GameplayStatics.GetPlayerController` 0))))

(fn `IndicateHit`
  (bind _character_wizard_01 (`self.Character_Wizard_01`))
  (`|SpawnActorFromClass` "/Game/Blueprints/Effects/BP_HitIndicator.BP_HitIndicator_C" (`KismetMathLibrary.MakeTransform` (+ (`SceneComponent.K2_GetComponentLocation` _character_wizard_01) (* (`SceneComponent.GetUpVector` _character_wizard_01) 100.0))) "Undefined" "OverrideRootScale" null null))

(fn `ShowCountdown`
  (`TextRenderComponent.K2_SetText` (`TextRenderActor.TextRender` (`self.CountdownActor`)) (`KismetTextLibrary.Conv_IntToText` (`KismetMathLibrary.FCeil` (`/Game/Blueprints/Gameplay/BP_GameState.Countdown` (`self.GameStateRef`))))))

(fn `ShowWidget`
  (params (ActorClass :type "Actor Class Reference"))
  (locals (UpDistance :type "Float (double-precision)" :default -10.0) (ForwardDistance :type "Float (double-precision)" :default 150.0))
  (bind _returnvalue_roll (`KismetMathLibrary.BreakRotator` (`self.K2_GetActorRotation`)))
  (bind _replicatedvrcamera (`self.ReplicatedVRCamera`))
  (bind (_returnvalue_roll_2 _returnvalue_pitch _returnvalue_yaw) (`KismetMathLibrary.BreakRotator` (`SceneComponent.K2_GetComponentRotation` _replicatedvrcamera)))
  (bind _returnvalue (`KismetMathLibrary.MakeRotator` 0.0 _returnvalue_pitch _returnvalue_yaw))
  (bind (_returnvalue_roll_3 _returnvalue_pitch_2 _returnvalue_yaw_2) (`KismetMathLibrary.BreakRotator` (`KismetMathLibrary.FindLookAtRotation` (`self.K2_GetActorLocation` (`self.WidgetActor`)) (`SceneComponent.K2_GetComponentLocation` (`self.ReplicatedVRCamera`)))))
  (bind _returnvalue_2 (`|SpawnActorFromClass` ActorClass (`KismetMathLibrary.MakeTransform` (0.0 0.0 0.0) (struct) (0.1 0.1 0.1)) "Undefined" "OverrideRootScale" null null))
  (bind _output_get (set `self.WidgetActor` _returnvalue_2))
  (`self.K2_SetActorLocation` _output_get (+ (`SceneComponent.K2_GetComponentLocation` _replicatedvrcamera) (+ (* (`KismetMathLibrary.GetForwardVector` _returnvalue) (`local.ForwardDistance`)) (* (`KismetMathLibrary.GetUpVector` _returnvalue) (`local.UpDistance`)))) false false)
  (`self.K2_SetActorRotation` _output_get (`KismetMathLibrary.MakeRotator` _returnvalue_roll _returnvalue_pitch_2 _returnvalue_yaw_2) false)
  (`SceneComponent.SetVisibility` (`Actor.RootComponent` (`self.WidgetActor`)) true false)
  (`self.K2_AttachToComponent` (`self.WidgetActor`) (`self.ReplicatedVRCamera`) "None" "KeepWorld" "KeepWorld" "KeepWorld" false))

(fn `StartCountdown`
  (locals (ForwardDistance :type "Float (double-precision)" :default 100.0))
  (bind _replicatedvrcamera (`self.ReplicatedVRCamera`))
  (bind _returnvalue (`SceneComponent.K2_GetComponentLocation` _replicatedvrcamera))
  (bind _returnvalue_2 (+ (* (`SceneComponent.GetForwardVector` _replicatedvrcamera) (`local.ForwardDistance`)) _returnvalue))
  (bind _returnvalue_3 (`|SpawnActorFromClass` "/Game/Blueprints/Characters/BP_Countdown.BP_Countdown_C" (`KismetMathLibrary.MakeTransform` _returnvalue_2 (`KismetMathLibrary.FindLookAtRotation` _returnvalue_2 _returnvalue)) "Undefined" "OverrideRootScale" null null))
  (bind _output_get (set `self.CountdownActor` _returnvalue_3))
  (`SceneComponent.K2_AttachToComponent` (`Actor.RootComponent` _output_get) (`self.ReplicatedVRCamera`) "None" "KeepWorld" "KeepWorld" "KeepWorld" true))

(fn `UpdateWizardTransform`
  (bind _returnvalue (`SceneComponent.K2_GetComponentToWorld` (`self.ReplicatedVRCamera`)))
  (bind _returnvalue_2 (`SceneComponent.K2_GetComponentToWorld` (`self.Character_Wizard_01`)))
  (`SceneComponent.K2_SetWorldLocationAndRotation` (`self.Character_Wizard_01`) (`KismetMathLibrary.MakeVector` (.x (.location _returnvalue)) (.y (.location _returnvalue)) (.z (.location _returnvalue_2))) (`KismetMathLibrary.MakeRotator` (.roll (.rotation _returnvalue_2)) (.pitch (.rotation _returnvalue_2)) (- (.yaw (.rotation _returnvalue)) 90.0)) false false))

(fn `UserConstructionScript`
  (set `self.VRBounds` (`SteamVRChaperoneComponent.GetBounds` (`self.SteamVRChaperone`))))