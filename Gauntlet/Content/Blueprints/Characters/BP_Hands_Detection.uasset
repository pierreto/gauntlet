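; VR player character with tracked hands that casts fireballs through right-hand gestures and quits the game when hit points run out.
; An open, upward hand spawns a fireball attached to the hand mesh; closing the fist replaces it with one launched at doubled, rolling-average hand velocity.
; Tick polls gestures, samples velocity and draws debug spheres for downward fists.
; BeginPlay hands both hands to SpellDetectionComponent; DisableMotionCapture reattaches meshes as a workaround.
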(event `self.ReceiveBeginPlay`
  (bind _spelldetectioncomponent (`self.SpellDetectionComponent`))
  ;[1 1 1] Set Character Start Attributes
  (`|ExecutionSequence`
    (:`then_0`
      (`HeadMountedDisplayFunctionLibrary.SetTrackingOrigin` "Floor")
      (set `self.HitPoints` 3.0))
    (:`then_1`
      (set `/Game/Blueprints/GestureSpells/SpellDetectionComponent.LeftHand` (`self.HandL`) _spelldetectioncomponent)
      (set `/Game/Blueprints/GestureSpells/SpellDetectionComponent.RightHand` (`self.HandR`) _spelldetectioncomponent))))

(event `self.ReceiveAnyDamage`
  (params (Damage :type "Float (single-precision)") (DamageType :type "DamageType Object Reference") (InstigatedBy :type "Controller Object Reference") (DamageCauser :type "Actor Object Reference"))
  ;[1 1 1] Damage
  (bind _output_get (set `self.HitPoints` (- (`self.HitPoints`) Damage)))
  (if (<= _output_get 0.0)
    (`KismetSystemLibrary.QuitGame` null "Quit")))

(event `self.ReceiveTick`
  (params (DeltaSeconds :type "Float (single-precision)"))
  (bind _handr (`self.HandR`))
  (bind _closedfistradius (`self.ClosedFistRadius`))
  (bind _handl (`self.HandL`))
  (bind _handr_2 (`self.HandR`))
  ;[1 1 1] Simple logic to spawn a fire ball when user opens hand
  (`|ExecutionSequence`
    (:`then_0`
      (`self.StoreRightHandVelocity` DeltaSeconds)
      (set `self.LastRightHandPos` (`SceneComponent.K2_GetComponentLocation` (`self.SkeletalMeshR`))))
    (:`then_1`
      (bind _isclosed (`/Game/Blueprints/GestureSpells/Hand.IsFistClosed` _handl))
      (bind _ispointingdown (`/Game/Blueprints/GestureSpells/Hand.HandPointingDown` _handl))
      (if (and _ispointingdown _isclosed)
        (bind _center (`/Game/Blueprints/GestureSpells/Hand.GetHandCenter` _handl))
        (`KismetSystemLibrary.DrawDebugSphere` _center _closedfistradius 20 (struct :`R` 1.0 :`A` 1.0))))
    (:`then_2`
      (bind _isclosed_2 (`/Game/Blueprints/GestureSpells/Hand.IsFistClosed` _handr))
      (bind _ispointingdown_2 (`/Game/Blueprints/GestureSpells/Hand.HandPointingDown` _handr))
      (if (and _ispointingdown_2 _isclosed_2)
        (bind _center_2 (`/Game/Blueprints/GestureSpells/Hand.GetHandCenter` _handr))
        (`KismetSystemLibrary.DrawDebugSphere` _center_2 _closedfistradius 20 (struct :`R` 1.0 :`A` 1.0))))
    (:`then_3`
      (bind _isopened (`/Game/Blueprints/GestureSpells/Hand.IsHandOpen` _handr_2))
      (bind _ispointingdown_3 (`/Game/Blueprints/GestureSpells/Hand.HandPointingUp` _handr_2))
      (if (and _ispointingdown_3 _isopened)
        (if (not (`self.HasFireBall_R`))
          (set `self.HasFireBall_R` true)
          (`self.SpawnFireball`))))
    (:`then_4`
      (bind _isclosed_3 (`/Game/Blueprints/GestureSpells/Hand.IsFistClosed` _handr_2))
      (if _isclosed_3
        (if (`self.HasFireBall_R`)
          (set `self.HasFireBall_R` false)
          (`self.ShootFireBallServer` (* (`KismetMathLibrary.GetVectorArrayAverage` (`self.RightHandVelocities`)) 2) (`SceneComponent.K2_GetComponentToWorld` (`self.SkeletalMeshR`))))))))

(event `InputAction|Exit`
  (params (Key :type "Key Structure"))
  ;[1 1 1] Simple logic to spawn a fire ball when user opens hand
  ;;[1 1 1] Quit
  (:`Pressed`
    (`KismetSystemLibrary.QuitGame` null "Quit")))

(event `SpawnFireball`
  ;[1 1 1] Fait apparaitre une boule de feu au dessus de la main
  (bind _returnvalue (`|SpawnActorFromClass` (`self.SpellToSpawn`) (`SceneComponent.K2_GetComponentToWorld` (`self.SkeletalMeshR`)) "AlwaysSpawn" "OverrideRootScale" null null))
  (`SceneComponent.K2_AddRelativeLocation` (`/Game/Blueprints/GestureSpells/Spells/BP_Fireball.Fire Ball` _returnvalue) (1.0 7.0 -10.0) false false)
  (`self.AttachFireball` _returnvalue))

(event `AttachFireball`
  (params (FireBall :type "/Game/Blueprints/GestureSpells/Spells/BP_Fireball Object Reference"))
  ;[1 1 1] Attach fireball multicast
  (bind _output_get (set `self.HeldFireBall_R` FireBall))
  (`SceneComponent.K2_AttachToComponent` (`/Game/Blueprints/GestureSpells/Spells/BP_Fireball.Fire Ball` _output_get) (`self.SkeletalMeshR`) "None" "KeepRelative" "KeepRelative" "KeepRelative" false))

(event `ShootFireBallServer`
  (params (HandVelocityAverage :type "Vector Structure") (HandTransform :type "Transform Structure"))
  (bind _heldfireball_r (`self.HeldFireBall_R`))
  ;[1 1 1] Shoot
  (if (`KismetSystemLibrary.IsValid` _heldfireball_r)
    (`self.K2_DestroyActor` _heldfireball_r)
    (bind _returnvalue (`|SpawnActorFromClass` (`self.SpellToSpawn`) HandTransform "AlwaysSpawn" "OverrideRootScale" null null))
    (`SceneComponent.K2_AddRelativeLocation` (`/Game/Blueprints/GestureSpells/Spells/BP_Fireball.Fire Ball` _returnvalue) (1.0 7.0 -10.0) false false)
    (`/Game/Blueprints/GestureSpells/Spells/BP_Fireball.SetVelocity` _returnvalue HandVelocityAverage)))

(fn `DisableMotionCapture`
  (bind _skeletalmeshr (`self.SkeletalMeshR`))
  (bind _skeletalmeshl (`self.SkeletalMeshL`))
  ;[1 1 1] Workaround To Fix Hands That Control Ze World. -- Vincent et Fabrice
  (`SceneComponent.K2_DetachFromComponent` _skeletalmeshr "KeepRelative" "KeepRelative" "KeepRelative" true)
  (`SceneComponent.K2_AttachToComponent` _skeletalmeshr (`self.HandR`) "None" "KeepRelative" "KeepRelative" "KeepRelative" false)
  (`SceneComponent.K2_DetachFromComponent` _skeletalmeshl "KeepRelative" "KeepRelative" "KeepRelative" true)
  (`SceneComponent.K2_AttachToComponent` _skeletalmeshl (`self.HandL`) "None" "KeepRelative" "KeepRelative" "KeepRelative" true))

(fn `StoreRightHandVelocity`
  (params (deltaT :type "Float (double-precision)"))
  (bind _righthandvelocities (`self.RightHandVelocities`))
  ;[1 1 1] Store Right Hand Velocity To Compute Average Later
  (`KismetArrayLibrary.Array_Add` _righthandvelocities (/ (- (`SceneComponent.K2_GetComponentLocation` (`self.SkeletalMeshR`)) (`self.LastRightHandPos`)) deltaT))
  (if (>= (`KismetArrayLibrary.Array_Length` _righthandvelocities) 10)
    (`KismetArrayLibrary.Array_Remove` (`self.RightHandVelocities`))))

(fn `UserConstructionScript`
  (set `self.VRBounds` (`SteamVRChaperoneComponent.GetBounds` (`self.SteamVRChaperone`))))