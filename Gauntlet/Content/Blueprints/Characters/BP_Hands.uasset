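; BP_Hands is the networked VR player pawn for a wizard duel with gesture-based hand controls.
; Tick moves the wizard body under the camera, feeds its AnimBP, and switches between gesture handling and countdown by game state.
; Threshold-gated speed and hand updates limit network traffic, with OnRep functions applying them.
; It also handles damage, spawned health-point actors, victory/defeat widgets, restart and tutorial inputs, and debug keys.
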(event `GameEnded`
  (params (Winner :type "Pawn Object Reference (by ref)"))
  ;[1 1 1] Show end game client
  (`self.CreateEndGameWidget` (not (== Winner self))))

(event `InputAction|StartTutoriel`
  (params (Key :type "Key Structure"))
  ;[1 1 1] Start Tutorial when key pressed
  (:`Pressed`
    (bind _outactors (`GameplayStatics.GetAllActorsOfClass` "/Game/Blueprints/Characters/BP_Tutorial.BP_Tutorial_C"))
    (bind _output (`|GetArrayItem` _outactors))
    (if (`KismetSystemLibrary.IsValid` _output)
      (`/Game/Blueprints/Characters/BP_Tutorial.StartTutorial` _output))))

(event `self.ReceiveBeginPlay`
  (bind _replicatedvrcamera (`self.ReplicatedVRCamera`))
  ;[1 1 1] Set Character Start Attributes
  (bind _asbp_game_state (cast `/Game/Blueprints/Gameplay/BP_GameState` (`GameplayStatics.GetGameState`)))
  (set `self.GameStateRef` _asbp_game_state)
  (`HeadMountedDisplayFunctionLibrary.SetTrackingOrigin` "Floor")
  (set `/Game/Blueprints/GestureSpells/Hand.VRCameraRef` _replicatedvrcamera (`self.HandR`))
  (set `/Game/Blueprints/GestureSpells/Hand.VRCameraRef` _replicatedvrcamera (`self.HandL`))
  (`/Engine/EditorBlueprintResources/ActorMacros.Switch Has Authority`
    (:`Authority`
      (`self.CreateHpActors`))))

(event `InputAction|RestartLevel`
  (params (Key :type "Key Structure"))
  ;[1 1 1] Restart Level
  (:`Pressed`
    (bind _asbp_game_state (cast `/Game/Blueprints/Gameplay/BP_GameState` (`GameplayStatics.GetGameState`)))
    (switch `/Game/Blueprints/Gameplay/EArenaGameStates` (`/Game/Blueprints/Gameplay/BP_GameState.GameState` _asbp_game_state)
      (:`NewEnumerator2`
        (`/Engine/EditorBlueprintResources/ActorMacros.Switch Has Authority`
          (:`Authority`
            (`self.GameRestartRequested`)
            (`self.RestartClient`)))))))

(event `self.ReceiveAnyDamage`
  (params (Damage :type "Float (single-precision)") (DamageType :type "DamageType Object Reference") (InstigatedBy :type "Controller Object Reference") (DamageCauser :type "Actor Object Reference"))
  ;[1 1 1] Damage
  (`self.IndicateHit`)
  (`self.RemoteTakeAnyDamage`)
  (if (not (`self.Invincible`))
    (set `self.HitPoints` (- (`self.HitPoints`) Damage))
    (`self.DestroyHpActor`)))

(event `RestartClient`
  ;[1 1 1] Restart Level
  (`self.DestroyWidget`))

(event `InputAction|Exit`
  (params (Key :type "Key Structure"))
  ;[1 1 1] Quit
  (:`Pressed`
    (`KismetSystemLibrary.QuitGame` null "Quit")))

(event `InputAction|BackToTutorial`
  (params (Key :type "Key Structure"))
  ;[1 1 1] Restart to tutorial
  (:`Pressed`
    (bind _asbp_game_state (cast `/Game/Blueprints/Gameplay/BP_GameState` (`GameplayStatics.GetGameState`)))
    (switch `/Game/Blueprints/Gameplay/EArenaGameStates` (`/Game/Blueprints/Gameplay/BP_GameState.GameState` _asbp_game_state)
      (:`NewEnumerator2`
        (`self.OpenTutorial`)))))

(event `OpenTutorial`
  ;[1 1 1] Restart to tutorial
  (`GameplayStatics.OpenLevel` "ArenaTutorial"))

(event `self.ReceiveTick`
  (params (DeltaSeconds :type "Float (single-precision)"))
  (bind _handr (`self.HandR`))
  (bind _handl (`self.HandL`))
  (`self.SetAnimHeight`)
  ;[1 1 1] Move Wizard
  (`self.UpdateWizardTransform`)
  (if (`self.HasOwnership`)
    (switch `/Game/Blueprints/Gameplay/EArenaGameStates` (`/Game/Blueprints/Gameplay/BP_GameState.GameState` (`self.GameStateRef`))
      (:`NewEnumerator3`
        ;[1 1 1] Detect gestures
        (`/Game/Blueprints/GestureSpells/Hand.HandleRightGesture` _handr DeltaSeconds :!label _label)
        (`/Game/Blueprints/GestureSpells/Hand.HandleAnyGesture` _handr DeltaSeconds)
        (`/Game/Blueprints/GestureSpells/Hand.HandleLeftGesture` _handl DeltaSeconds)
        (`/Game/Blueprints/GestureSpells/Hand.HandleAnyGesture` _handl DeltaSeconds))
      (:`NewEnumerator4`
        ;[1 1 1] Show countdown
        (`/Engine/EditorBlueprintResources/StandardMacros.IsValid` (`self.CountdownActor`)
          (:`Is Valid`
            (`self.ShowCountdown`))
          (:`Is Not Valid`
            (`self.StartCountdown`))))
      (:`NewEnumerator1`
        ;[1 1 1] Hide countdown
        (`/Engine/EditorBlueprintResources/StandardMacros.IsValid` (`self.CountdownActor`)
          (:`Is Valid`
            (`self.K2_DestroyActor` (`self.CountdownActor`))
            (goto _label))
          (:`Is Not Valid`
            (goto _label)))))))

(event `Key|H`
  (params (Key :type "Key Structure"))
  ;[1 1 1] Damage
  (:`Pressed`
    (`GameplayStatics.ApplyDamage` self 1.0)))

(event `RemoteTakeAnyDamage`
  ;[1 1 1] Damage
  (bind _ashit_effect (cast `/Game/Blueprints/Widgets/HitEffect` (`WidgetComponent.GetUserWidgetObject` (`self.HUDWidget`))))
  (`/Game/Blueprints/Widgets/HitEffect.TakeDamage` _ashit_effect))

(event `Key|S`
  (params (Key :type "Key Structure"))
  ;[1 1 1] Skip tutorial
  (:`Released`
    (bind _outactors (`GameplayStatics.GetAllActorsOfClass` "/Game/Blueprints/Characters/BP_Tutorial.BP_Tutorial_C"))
    (`/Game/Blueprints/Characters/BP_Tutorial.SkipTutorial` (`|GetArrayItem` _outactors))))

(event `Key|A`
  (params (Key :type "Key Structure"))
  ;[1 1 1] Test end game sequence
  (:`Released`
    (`self.GameEndedServer`)))

(event `GameEndedServer`
  ;[1 1 1] Test end game sequence
  (bind _asbp_rounds_game_mode (cast `/Game/Blueprints/Gameplay/Bp_RoundsGameMode` (`GameplayStatics.GetGameMode`)))
  (`/Game/Blueprints/Gameplay/BP_GymGameMode.OnGameEnded` _asbp_rounds_game_mode self))

(fn `CreateEndGameWidget`
  (params (HasLost :type Boolean))
  (if HasLost
    (`self.ShowWidget` "/Game/Blueprints/Widgets/BP_Defeat.BP_Defeat_C")
    (else
      (`self.ShowWidget` "/Game/Blueprints/Widgets/BP_Victory.BP_Victory_C"))))

(fn `CreateHpActors`
  (bind _output_get (set `self.HitPoints` (`self.HitPoints`)))
  (bind _closestactor (`self.GetClosestActor` "/Script/Engine.PlayerStart"))
  (for _index (range 1 (+ (`KismetMathLibrary.FTrunc` _output_get) 1))
    (bind _returnvalue (`|SpawnActorFromClass` "/Game/Blueprints/BP_HealthPoint.BP_HealthPoint_C" (`self.DefaultTransform`) "AlwaysSpawn" "OverrideRootScale" null null))
    (bind _rootcomponent (`Actor.RootComponent` _closestactor))
    (bind _returnvalue_2 (`SceneComponent.GetUpVector` _rootcomponent))
    (bind (_returnvalue_x _returnvalue_y _returnvalue_z) (`KismetMathLibrary.BreakVector` (+ (`SceneComponent.K2_GetComponentLocation` _rootcomponent) (* _returnvalue_2 20) (* _returnvalue_2 (* _index (`self.HorizontalHpOffset`))) (* _returnvalue_2 (/ (* (+ _output_get 1.0) (`self.HorizontalHpOffset`)) -2.0)) (100.0 0.0 0.0) (* (`SceneComponent.GetForwardVector` _rootcomponent) 150.0))))
    (`self.K2_SetActorLocation` _returnvalue (`KismetMathLibrary.MakeVector` _returnvalue_x (* _returnvalue_y 0.7) _returnvalue_z) false false)
    (`KismetArrayLibrary.Array_Add` (`self.HpActors`) _returnvalue)))

(fn `DestroyAttachedWidget`
  (params (WidgetClass :type "Actor Class Reference"))
  (bind _outactors (`GameplayStatics.GetAllActorsOfClass` WidgetClass))
  (for _array_element _outactors
    (`self.K2_DetachFromActor` _array_element "KeepRelative" "KeepRelative" "KeepRelative")
    (`self.K2_DestroyActor` _array_element)))

(fn `DestroyHpActor`
  (bind _returnvalue (`KismetArrayLibrary.Array_Length` (`self.HpActors`)))
  (bind _returnvalue_2 (- _returnvalue 1))
  (if (> _returnvalue 0)
    (`/Game/Blueprints/BP_HealthPoint.OnHpRemoved` (`|GetArrayItem` (`self.HpActors`) _returnvalue_2))
    (`KismetArrayLibrary.Array_Remove` (`self.HpActors`) _returnvalue_2)))

(fn `DestroyWidget`
  (bind _outactors (`GameplayStatics.GetAllActorsOfClass` "/Game/Blueprints/Widgets/BP_Defeat.BP_Defeat_C"))
  (for _array_element _outactors
    (`self.K2_DetachFromActor` _array_element "KeepRelative" "KeepRelative" "KeepRelative")
    (`self.K2_DestroyActor` _array_element))
  (bind _outactors_2 (`GameplayStatics.GetAllActorsOfClass` "/Game/Blueprints/Widgets/BP_Victory.BP_Victory_C"))
  (for _array_element_2 _outactors_2
    (`self.K2_DetachFromActor` _array_element_2 "KeepRelative" "KeepRelative" "KeepRelative")
    (`self.K2_DestroyActor` _array_element_2)))

(fn `GetClosestActor`
  (params (ObjectClass :type "Actor Class Reference"))
  (returns (ClosestActor :type "Actor Object Reference"))
  (locals (smallestDistance :type "Float (double-precision)" :default 999999.0) (closeActor :type "Actor Object Reference"))
  (bind _outactors (`GameplayStatics.GetAllActorsOfClass` ObjectClass))
  (for _array_element _outactors
    (bind _returnvalue (`self.GetDistanceTo` _array_element))
    (if (< _returnvalue (`local.smallestDistance`))
      (set `local.closeActor` _array_element)
      (set `local.smallestDistance` _returnvalue)))
  (return (`local.closeActor`)))

(fn `GetFireballScale`)

(fn `HandleDoubleHandGestures`
  (params (DeltaTime :type "Float (double-precision)"))
  (returns (Detected :type Boolean))
  (locals (_Detected :type Boolean :default true))
  (bind _shootdirection (`self.DoubleHandGestures` DeltaTime)
    (:`OnShootFIreball`
      (`self.ShootFireballServer` _shootdirection))
    (:`OnFinalFireball`
      (`self.MoveDoubleFireball`))
    (:`OnGrowFireball`
      (`self.GrowFireball`))
    (:`OnStopFireball`
      (`self.CancelFireball`)
      (set `local._Detected` false :!label _label))
    (:`OnSpawnFireball`
      (`self.SpawnFireballDoubleHand`))
    (:`Other`
      (goto _label)))
  (return (`local._Detected`)))

(fn `HasOwnership`
  (returns (IsOwner :type Boolean))
  (return (== (`self.GetController`) (`GameplayStatics.GetPlayerController` 0))))

(fn `IndicateHit`
  (bind _character_wizard_01 (`self.Character_Wizard_01`))
  (`|SpawnActorFromClass` "/Game/Blueprints/Effects/BP_HitIndicator.BP_HitIndicator_C" (`KismetMathLibrary.MakeTransform` (+ (`SceneComponent.K2_GetComponentLocation` _character_wizard_01) (* (`SceneComponent.GetUpVector` _character_wizard_01) 100.0))) "Undefined" "OverrideRootScale" null null))

(fn `InitializeHeight`
  (set `self.Height` (- (.z (`SceneComponent.K2_GetComponentLocation` (`self.HeightPoint`))) (.z (`SceneComponent.K2_GetComponentLocation` (`self.CrouchPoint`))))))

(fn `OnRep_LeftHandColor`
  (bind _returnvalue (`PrimitiveComponent.CreateDynamicMaterialInstance` (`self.SkeletalMeshL`) 0 "/Game/Assets/Characters/Wizard_Material_Instance.Wizard_Material_Instance" "None"))
  (`MaterialInstanceDynamic.SetVectorParameterValue` _returnvalue "Color" (`self.LeftHandColor`)))

(fn `OnRep_LeftHandPos`
  (bind _asbp_wizard_anim (cast `/Game/Assets/Animation/BP_WizardAnim` (`SkeletalMeshComponent.GetAnimInstance` (`self.Character_Wizard_01`))))
  (set `/Game/Assets/Animation/BP_WizardAnim.LeftHandTarget` (`self.LeftHandPos`) _asbp_wizard_anim))

(fn `OnRep_PlayerColor`
  (bind _returnvalue (`PrimitiveComponent.CreateDynamicMaterialInstance` (`self.Character_Wizard_01`) 0 "/Game/Assets/Characters/Wizard_Material_Instance.Wizard_Material_Instance" "None"))
  (`MaterialInstanceDynamic.SetVectorParameterValue` _returnvalue "Color" (`self.PlayerColor`)))

(fn `OnRep_PlayerHorizontalSpeed`
  (bind _asbp_wizard_anim (cast `/Game/Assets/Animation/BP_WizardAnim` (`SkeletalMeshComponent.GetAnimInstance` (`self.Character_Wizard_01`))))
  (set `/Game/Assets/Animation/BP_WizardAnim.HorizontalSpeed` (`self.PlayerHorizontalSpeed`) _asbp_wizard_anim))

(fn `OnRep_RightHandColor`
  (bind _returnvalue (`PrimitiveComponent.CreateDynamicMaterialInstance` (`self.SkeletalMeshR`) 0 "/Game/Assets/Characters/Wizard_Material_Instance.Wizard_Material_Instance" "None"))
  (`MaterialInstanceDynamic.SetVectorParameterValue` _returnvalue "Color" (`self.RightHandColor`)))

(fn `OnRep_RightHandPos`
  (bind _asbp_wizard_anim (cast `/Game/Assets/Animation/BP_WizardAnim` (`SkeletalMeshComponent.GetAnimInstance` (`self.Character_Wizard_01`))))
  (set `/Game/Assets/Animation/BP_WizardAnim.RightHandTarget` (`self.RightHandPos`) _asbp_wizard_anim))

(fn `SetAnimHeight`
  (bind _asbp_wizard_anim (cast `/Game/Assets/Animation/BP_WizardAnim` (`SkeletalMeshComponent.GetAnimInstance` (`self.Character_Wizard_01`))))
  (set `/Game/Assets/Animation/BP_WizardAnim.CameraRHeight` (/ (- (.z (`SceneComponent.K2_GetComponentLocation` (`self.ReplicatedVRCamera`))) (.z (`SceneComponent.K2_GetComponentLocation` (`self.CrouchPoint`)))) (`self.Height`)) _asbp_wizard_anim))

(fn `SetAnimWalkSpeed`
  (params (Speed :type "Float (double-precision)") (isowner :type Boolean))
  (bind _asbp_wizard_anim (cast `/Game/Assets/Animation/BP_WizardAnim` (`SkeletalMeshComponent.GetAnimInstance` (`self.Character_Wizard_01`))))
  (bind _output_get (set `/Game/Assets/Animation/BP_WizardAnim.HorizontalSpeed` Speed _asbp_wizard_anim))
  (if (not isowner)
    (`KismetSystemLibrary.PrintString` (`KismetStringLibrary.Conv_DoubleToString` _output_get) true true (struct :`G` 0.66 :`B` 1.0 :`A` 1.0) 202.0)))

(fn `ShowCountdown`
  (`TextRenderComponent.K2_SetText` (`TextRenderActor.TextRender` (`self.CountdownActor`)) (`KismetTextLibrary.Conv_IntToText` (`KismetMathLibrary.FCeil` (`/Game/Blueprints/Gameplay/BP_GameState.Countdown` (`self.GameStateRef`))))))

(fn `ShowWidget`
  (params (ActorClass :type "Actor Class Reference"))
  (returns (CreatedWidget :type "Actor Object Reference"))
  (locals (UpDistance :type "Float (double-precision)" :default -10.0) (ForwardDistance :type "Float (double-precision)" :default 150.0))
  (bind _returnvalue_roll (`KismetMathLibrary.BreakRotator` (`self.K2_GetActorRotation`)))
  (bind _replicatedvrcamera (`self.ReplicatedVRCamera`))
  (bind (_returnvalue_roll_2 _returnvalue_pitch _returnvalue_yaw) (`KismetMathLibrary.BreakRotator` (`SceneComponent.K2_GetComponentRotation` _replicatedvrcamera)))
  (bind _returnvalue (`KismetMathLibrary.MakeRotator` 0.0 _returnvalue_pitch _returnvalue_yaw))
  (bind (_returnvalue_roll_3 _returnvalue_pitch_2 _returnvalue_yaw_2) (`KismetMathLibrary.BreakRotator` (`KismetMathLibrary.FindLookAtRotation` (`self.K2_GetActorLocation` (`self.WidgetActor`)) (`SceneComponent.K2_GetComponentLocation` (`self.ReplicatedVRCamera`)))))
  (bind _returnvalue_2 (`|SpawnActorFromClass` ActorClass (`KismetMathLibrary.MakeTransform` (0.0 0.0 0.0) (struct) (0.1 0.1 0.1)) "Undefined" "OverrideRootScale" null null))
  (bind _output_get (set `self.WidgetActor` _returnvalue_2))
  (`self.K2_SetActorLocation` _output_get (+ (`SceneComponent.K2_GetComponentLocation` _replicatedvrcamera) (+ (* (`KismetMathLibrary.GetForwardVector` _returnvalue) (`local.ForwardDistance`)) (* (`KismetMathLibrary.GetUpVector` _returnvalue) (`local.UpDistance`)))) false false)
  (`self.K2_SetActorRotation` _output_get (`KismetMathLibrary.MakeRotator` _returnvalue_roll _returnvalue_pitch_2 _returnvalue_yaw_2) false)
  (`SceneComponent.SetVisibility` (`Actor.RootComponent` (`self.WidgetActor`)) true false)
  (`self.K2_AttachToComponent` (`self.WidgetActor`) (`self.ReplicatedVRCamera`) "None" "KeepWorld" "KeepWorld" "KeepWorld" false)
  (return _returnvalue_2))

(fn `StartCountdown`
  (locals (ForwardDistance :type "Float (double-precision)" :default 100.0))
  (bind _replicatedvrcamera (`self.ReplicatedVRCamera`))
  (bind _returnvalue (`SceneComponent.K2_GetComponentLocation` _replicatedvrcamera))
  (bind _returnvalue_2 (+ (* (`SceneComponent.GetForwardVector` _replicatedvrcamera) (`local.ForwardDistance`)) _returnvalue))
  (bind _returnvalue_3 (`|SpawnActorFromClass` "/Game/Blueprints/Characters/BP_Countdown.BP_Countdown_C" (`KismetMathLibrary.MakeTransform` _returnvalue_2 (`KismetMathLibrary.FindLookAtRotation` _returnvalue_2 _returnvalue)) "Undefined" "OverrideRootScale" null null))
  (bind _output_get (set `self.CountdownActor` _returnvalue_3))
  (`SceneComponent.K2_AttachToComponent` (`Actor.RootComponent` _output_get) (`self.ReplicatedVRCamera`) "None" "KeepWorld" "KeepWorld" "KeepWorld" true))

(fn `UpdateWizardTransform`
  (bind _returnvalue (`SceneComponent.K2_GetComponentToWorld` (`self.ReplicatedVRCamera`)))
  (bind _returnvalue_2 (`SceneComponent.K2_GetComponentToWorld` (`self.Character_Wizard_01`)))
  (bind _returnvalue_3 (`SceneComponent.K2_GetComponentToWorld` (`self.SkeletalMeshL`)))
  (bind _returnvalue_4 (`SceneComponent.K2_GetComponentToWorld` (`self.SkeletalMeshR`)))
  (bind _returnvalue_5 (- (.x (.location _returnvalue_2)) (.x (.location _returnvalue))))
  ;[1 1 1] Set horizontal delta value if delta is above threshold to limit net calls and stutters
  (`|ExecutionSequence`
    (:`then_0`
      (if (> (`KismetMathLibrary.Abs` _returnvalue_5) (`self.NetworkSpeedThreshold`))
        (set `self.PlayerHorizontalSpeed` (* _returnvalue_5 -1.0))))
    (:`then_1`
      (`SceneComponent.K2_SetWorldLocationAndRotation` (`self.Character_Wizard_01`) (`KismetMathLibrary.MakeVector` (.x (.location _returnvalue)) (.y (.location _returnvalue)) (.z (.location _returnvalue_2))) (`KismetMathLibrary.MakeRotator` (.roll (.rotation _returnvalue_2)) (.pitch (.rotation _returnvalue_2)) (- (.yaw (.rotation _returnvalue)) 90.0)) false false))
    (:`then_2`
      (if (> (`KismetMathLibrary.VSize` (- (.location _returnvalue_3) (.location (`self.LeftHandPos`)))) (`self.NetworkSpeedThreshold`))
        (set `self.LeftHandPos` _returnvalue_3)))
    (:`then_3`
      (if (> (`KismetMathLibrary.VSize` (- (.location _returnvalue_4) (.location (`self.RightHandPos`)))) (`self.NetworkSpeedThreshold`))
        (set `self.RightHandPos` _returnvalue_4)))))

(fn `UserConstructionScript`
  (set `self.VRBounds` (`SteamVRChaperoneComponent.GetBounds` (`self.SteamVRChaperone`)))
  (bind _returnvalue (`PrimitiveComponent.CreateDynamicMaterialInstance` (`self.Character_Wizard_01`) 0 "/Game/Assets/Characters/Wizard_Material_Instance.Wizard_Material_Instance" "None"))
  (bind _output_get (set `self.ColorMaterial` _returnvalue))
  (`MaterialInstanceDynamic.SetVectorParameterValue` _output_get "Color" (struct :`R` 1.0 :`G` 1.0 :`B` 1.0 :`A` 1.0))
  (`self.InitializeHeight`))