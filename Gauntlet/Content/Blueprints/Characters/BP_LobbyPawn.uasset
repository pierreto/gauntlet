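; BP_LobbyPawn is the lobby pawn that lets the player host or join a game session through input actions.
; On BeginPlay it caches BP_GameInstance, and the Host and Join presses forward to its HostGame and JoinGame functions.
; ShowMenuWidget, not called within this Blueprint, spawns a scaled-down BP_MenuActor at the world origin.
; Its logic for placing and attaching a widget relative to the VR camera is disconnected and never runs.
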(event `self.ReceiveBeginPlay`
  ;[1 1 1] Begin and set GameInstaceRef
  (bind _asbp_game_instance (cast `/Game/Blueprints/Gameplay/BP_GameInstance` (`GameplayStatics.GetGameInstance`)))
  (set `self.GameInstanceRef` _asbp_game_instance))

(event `InputAction|Host`
  (params (Key :type "Key Structure"))
  ;[1 1 1] Host Session
  (:`Pressed`
    (`/Game/Blueprints/Gameplay/BP_GameInstance.HostGame` (`self.GameInstanceRef`))))

(event `InputAction|Join`
  (params (Key :type "Key Structure"))
  ;[1 1 1] Join Session
  (:`Pressed`
    (`/Game/Blueprints/Gameplay/BP_GameInstance.JoinGame` (`self.GameInstanceRef`))))

(fn `ShowMenuWidget`
  (bind _returnvalue (`|SpawnActorFromClass` "/Game/Blueprints/Widgets/BP_MenuActor.BP_MenuActor_C" (`KismetMathLibrary.MakeTransform` (0.0 0.0 0.0) (struct) (0.1 0.1 0.1)) "Undefined" "OverrideRootScale" null null))
  (cast `/Game/Blueprints/Widgets/BP_MenuActor` _returnvalue))

(fn `UserConstructionScript`)