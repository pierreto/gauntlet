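; VR wizard character that can record and replay hand gestures, with hit points and an end-game screen.
; Tick records hand socket transforms to a save game, or draws fist debug spheres and aligns the wizard body to the headset.
; Playback is unfinished: it only reads the first frame and never applies sockets.
; Damage removes spawned health-point actors, and game mode's game-ended event shows a camera-attached victory or defeat widget.
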(event `self.ReceiveBeginPlay`
  ;[1 1 1] Set Character Start Attributes
  (bind _asbp_gym_game_mode (cast `/Game/Blueprints/Gameplay/BP_GymGameMode` (`GameplayStatics.GetGameMode`)))
  (add `/Game/Blueprints/Gameplay/BP_GymGameMode.OnGameEnded` _asbp_gym_game_mode (delegate `GameEnded`))
  (`HeadMountedDisplayFunctionLibrary.SetTrackingOrigin` "Floor")
  (`/Engine/EditorBlueprintResources/ActorMacros.Switch Has Authority`
    (:`Authority`
      (`self.CreateHpActors`))))

(event `GameEnded`
  (`self.ShowEndGameClient`))

(event `ShowEndGameClient`
  (bind _hitpoints (`self.HitPoints`))
  (`KismetSystemLibrary.PrintString` (`KismetStringLibrary.Conv_DoubleToString` _hitpoints) true true (struct :`G` 0.66 :`B` 1.0 :`A` 1.0) 10000.0)
  (`self.CreateEndGameWidget` (< _hitpoints 1.0)))

(event `self.ReceiveAnyDamage`
  (params (Damage :type "Float (single-precision)") (DamageType :type "DamageType Object Reference") (InstigatedBy :type "Controller Object Reference") (DamageCauser :type "Actor Object Reference"))
  ;[1 1 1] Damage
  (set `self.HitPoints` (- (`self.HitPoints`) Damage))
  (`self.DestroyHpActor`))

(event `self.ReceiveTick`
  (params (DeltaSeconds :type "Float (single-precision)"))
  (bind _handr (`self.HandR`))
  (bind _closedfistradius (`self.ClosedFistRadius`))
  (bind _handl (`self.HandL`))
  ;[1 1 1] Simple logic to spawn a fire ball when user opens hand
  (`|ExecutionSequence`
    (:`then_0`
      (if (`self.IsRecordingGesture`)
        (`self.RecordGesture` DeltaSeconds)
        (else
          (`|ExecutionSequence` :!label _label
            (:`then_0`
              (bind _isclosed (`/Game/Blueprints/GestureSpells/Hand.IsFistClosed` _handl))
              (bind _ispointingdown (`/Game/Blueprints/GestureSpells/Hand.HandPointingDown` _handl))
              (if (and _ispointingdown _isclosed)
                (bind _center (`/Game/Blueprints/GestureSpells/Hand.GetHandCenter` _handl))
                (`KismetSystemLibrary.DrawDebugSphere` _center _closedfistradius 20 (struct :`R` 1.0 :`A` 1.0))))
            (:`then_1`
              (bind _isclosed_2 (`/Game/Blueprints/GestureSpells/Hand.IsFistClosed` _handr))
              (bind _ispointingdown_2 (`/Game/Blueprints/GestureSpells/Hand.HandPointingDown` _handr))
              (if (and _ispointingdown_2 _isclosed_2)
                (bind _center_2 (`/Game/Blueprints/GestureSpells/Hand.GetHandCenter` _handr))
                (`KismetSystemLibrary.DrawDebugSphere` _center_2 _closedfistradius 20 (struct :`R` 1.0 :`A` 1.0))))
            (:`then_3`
              (`self.UpdateWizardTransform`))))))
    (:`then_1`
      (if (`self.IsPlayingRecording`)
        (`self.PlayRecording` (`self.Recordings`) DeltaSeconds)
        (else
          (goto _label))))))

(event `InputAction|Exit`
  (params (Key :type "Key Structure"))
  ;[1 1 1] Quit
  (:`Pressed`
    (`KismetSystemLibrary.QuitGame` null "Quit")))

(event `ReplicateHandTransform`
  (params (SkeletalMeshR :type "SkeletalMeshComponent Object Reference") (HandTransform :type "Transform Structure"))
  ;[1 1 1] Replicate hand transform from client to server
  ;;[1 1 1] Replicate on each Tick seems a little overkill and might cause network issues
  (`SceneComponent.K2_SetWorldTransform` SkeletalMeshR HandTransform false false))

(event `InputAction|RecordGesture`
  (params (Key :type "Key Structure"))
  (bind _recordings (`self.Recordings`))
  ;[1 1 1] Start and stop recording
  (:`Released`
    (set `self.CurrentRecordTime` 0.0)
    (bind _output_get (set `self.IsRecordingGesture` (not (`self.IsRecordingGesture`))))
    (if (not _output_get)
      (`self.SaveRecording` _recordings))
    (`KismetArrayLibrary.Array_Clear` _recordings)))

(event `InputAction|PlayGesture`
  (params (Key :type "Key Structure"))
  ;[1 1 1] Load gesture recording and start playing
  (:`Released`
    (if (not (`self.IsRecordingGesture`))
      (bind _output_get (set `self.IsPlayingRecording` (not (`self.IsPlayingRecording`))))
      (if _output_get
        (bind _recordings (`self.LoadRecording` "TestSaveSlot"))
        (set `self.Recordings` _recordings)
        (set `self.CurrentReplayTime` 0.0)))))

(fn `CreateEndGameWidget`
  (params (HasLost :type Boolean))
  (if HasLost
    (`self.ShowWidget` "/Game/Blueprints/Widgets/BP_Defeat.BP_Defeat_C")
    (else
      (`self.ShowWidget` "/Game/Blueprints/Widgets/BP_Victory.BP_Victory_C"))))

(fn `CreateHpActors`
  (bind _character_wizard_01 (`self.Character_Wizard_01`))
  (bind _returnvalue (`SceneComponent.GetUpVector` _character_wizard_01))
  (bind _output_get (set `self.HitPoints` (`self.HitPoints`)))
  (for _index (range 1 (+ (`KismetMathLibrary.FTrunc` _output_get) 1))
    (bind _returnvalue_2 (`|SpawnActorFromClass` "/Game/Blueprints/BP_HealthPoint.BP_HealthPoint_C" (`self.DefaultTransform`) "AlwaysSpawn" "OverrideRootScale" null null))
    (`self.K2_SetActorLocation` _returnvalue_2 (+ (`SceneComponent.K2_GetComponentLocation` _character_wizard_01) (* _returnvalue 20) (* _returnvalue (* _index (`self.HorizontalHpOffset`))) (* _returnvalue (/ (* (+ _output_get 1.0) (`self.HorizontalHpOffset`)) -2.0)) (150.0 -150.0 0.0)) false false)
    (`KismetArrayLibrary.Array_Add` (`self.HpActors`) _returnvalue_2)))

(fn `DestroyHpActor`
  (bind _hpactors (`self.HpActors`))
  (bind _returnvalue (- (`KismetArrayLibrary.Array_Length` _hpactors) 1))
  (`self.K2_DestroyActor` (`|GetArrayItem` _hpactors _returnvalue))
  (`KismetArrayLibrary.Array_Remove` _hpactors _returnvalue))

(fn `DisableMotionCapture`
  (bind _skeletalmeshr (`self.SkeletalMeshR`))
  (bind _skeletalmeshl (`self.SkeletalMeshL`))
  ;[1 1 1] Workaround To Fix Hands That Control Ze World. -- Vincent et Fabrice
  (`SceneComponent.K2_DetachFromComponent` _skeletalmeshr "KeepRelative" "KeepRelative" "KeepRelative" true)
  (`SceneComponent.K2_AttachToComponent` _skeletalmeshr (`self.HandR`) "None" "KeepRelative" "KeepRelative" "KeepRelative" false)
  (`SceneComponent.K2_DetachFromComponent` _skeletalmeshl "KeepRelative" "KeepRelative" "KeepRelative" true)
  (`SceneComponent.K2_AttachToComponent` _skeletalmeshl (`self.HandL`) "None" "KeepRelative" "KeepRelative" "KeepRelative" true))

(fn `GetHandTransforms`
  (params (HandSKM :type "SceneComponent Object Reference"))
  (returns (HandTransforms :type "Array of Transform Structure"))
  (locals (SkeletalMesh :type "SceneComponent Object Reference") (Transforms :type "Array of Transform Structure"))
  (bind _output_get (set `local.SkeletalMesh` HandSKM))
  (for _array_element (`SceneComponent.GetAllSocketNames` _output_get)
    (`KismetArrayLibrary.Array_Add` (`local.Transforms`) (`SceneComponent.GetSocketTransform` (`local.SkeletalMesh`) _array_element "RTS_World")))
  (return (`local.Transforms`)))

(fn `LoadRecording`
  (params (SaveSlot :type String))
  (returns (Recordings :type "Array of /Game/Blueprints/Dev/GestureRecording Structure"))
  (`KismetSystemLibrary.PrintString` "Loading...")
  (`GameplayStatics.CreateSaveGameObject` "/Game/Blueprints/Dev/RecordingSaveGame.RecordingSaveGame_C")
  (bind _returnvalue (`GameplayStatics.LoadGameFromSlot` SaveSlot))
  (bind _asrecording_save_game (cast `/Game/Blueprints/Dev/RecordingSaveGame` _returnvalue))
  (bind _recordings (`/Game/Blueprints/Dev/RecordingSaveGame.Recordings` _asrecording_save_game))
  (`KismetSystemLibrary.PrintString` (`KismetStringLibrary.Concat_StrStr` "Loaded : " (`KismetStringLibrary.Conv_IntToString` (`KismetArrayLibrary.Array_Length` _recordings)) " recordings!"))
  (return _recordings))

(fn `PlayRecording`
  (params (Recordings :type "Array of /Game/Blueprints/Dev/GestureRecording Structure") (DeltaTime :type "Float (double-precision)"))
  (bind (_lefthandsockets _righthandsockets _recordtime) (break `/Game/Blueprints/Dev/GestureRecording` (`|GetArrayItem` Recordings)))
  (bind _output_get (set `self.CurrentReplayTime` (+ DeltaTime (`self.CurrentReplayTime`))))
  (if (>= _output_get _recordtime)
    (`self.SetHandSockets` _lefthandsockets (`self.SkeletalMeshL`))
    (`self.SetHandSockets` _righthandsockets (`self.SkeletalMeshR`))))

(fn `RecordGesture`
  (params (DeltaSeconds :type "Float (double-precision)"))
  (locals (Delta :type "Float (double-precision)"))
  (bind _output_get (set `local.Delta` DeltaSeconds))
  (set `self.CurrentRecordTime` (+ _output_get (`self.CurrentRecordTime`)))
  (bind _center (`/Game/Blueprints/GestureSpells/Hand.GetHandCenter` (`self.HandR`)))
  (`KismetSystemLibrary.DrawDebugSphere` _center 10.0 12 (struct :`R` 1.0 :`A` 1.0) -1.0)
  (bind _center_2 (`/Game/Blueprints/GestureSpells/Hand.GetHandCenter` (`self.HandL`)))
  (`KismetSystemLibrary.DrawDebugSphere` _center_2 10.0 12 (struct :`R` 1.0 :`A` 1.0) -1.0)
  (bind _handtransforms (`self.GetHandTransforms` (`self.SkeletalMeshR`)))
  (bind _handtransforms_2 (`self.GetHandTransforms` (`self.SkeletalMeshL`)))
  (`KismetArrayLibrary.Array_Add` (`self.Recordings`) (make `/Game/Blueprints/Dev/GestureRecording` _handtransforms_2 _handtransforms (`self.CurrentRecordTime`))))

(fn `SaveRecording`
  (params (Recording :type "Array of /Game/Blueprints/Dev/GestureRecording Structure"))
  (locals (Data :type "Array of String"))
  (`KismetSystemLibrary.PrintString` "Saving...")
  (bind _returnvalue (`GameplayStatics.CreateSaveGameObject` "/Game/Blueprints/Dev/RecordingSaveGame.RecordingSaveGame_C"))
  (bind _output_get (set `/Game/Blueprints/Dev/RecordingSaveGame.Recordings` Recording _returnvalue))
  (bind _returnvalue_2 (`GameplayStatics.SaveGameToSlot` _returnvalue (`/Game/Blueprints/Dev/RecordingSaveGame.SlotName` _returnvalue) (`/Game/Blueprints/Dev/RecordingSaveGame.UserIndex` _returnvalue)))
  (if _returnvalue_2
    (`KismetSystemLibrary.PrintString` (`KismetStringLibrary.Concat_StrStr` "Saved " (`KismetStringLibrary.Conv_IntToString` (`KismetArrayLibrary.Array_Length` _output_get)) " recordings!"))))

(fn `SetHandSockets`
  (params (SocketTransforms :type "Array of Transform Structure") (HandSKM :type "SceneComponent Object Reference"))
  (locals (Transforms :type "Array of Transform Structure"))
  (set `local.Transforms` SocketTransforms)
  (for _ (`SceneComponent.GetAllSocketNames` HandSKM)
    _))

(fn `ShowWidget`
  (params (ActorClass :type "Actor Class Reference"))
  (locals (UpDistance :type "Float (double-precision)" :default -10.0) (ForwardDistance :type "Float (double-precision)" :default 150.0))
  (bind _returnvalue_roll (`KismetMathLibrary.BreakRotator` (`self.K2_GetActorRotation`)))
  (bind _replicatedvrcamera (`self.ReplicatedVRCamera`))
  (bind (_returnvalue_roll_2 _returnvalue_pitch _returnvalue_yaw) (`KismetMathLibrary.BreakRotator` (`SceneComponent.K2_GetComponentRotation` _replicatedvrcamera)))
  (bind _returnvalue (`KismetMathLibrary.MakeRotator` 0.0 _returnvalue_pitch _returnvalue_yaw))
  (bind (_returnvalue_roll_3 _returnvalue_pitch_2 _returnvalue_yaw_2) (`KismetMathLibrary.BreakRotator` (`KismetMathLibrary.FindLookAtRotation` (`self.K2_GetActorLocation` (`self.WidgetActor`)) (`SceneComponent.K2_GetComponentLocation` (`self.ReplicatedVRCamera`)))))
  (bind _returnvalue_2 (`|SpawnActorFromClass` ActorClass (`KismetMathLibrary.MakeTransform` (0.0 0.0 0.0) (struct) (0.1 0.1 0.1)) "Undefined" "OverrideRootScale" null null))
  (bind _output_get (set `self.WidgetActor` _returnvalue_2))
  (`self.K2_SetActorLocation` _output_get (+ (`SceneComponent.K2_GetComponentLocation` _replicatedvrcamera) (+ (* (`KismetMathLibrary.GetForwardVector` _returnvalue) (`local.ForwardDistance`)) (* (`KismetMathLibrary.GetUpVector` _returnvalue) (`local.UpDistance`)))) false false)
  (`self.K2_SetActorRotation` _output_get (`KismetMathLibrary.MakeRotator` _returnvalue_roll _returnvalue_pitch_2 _returnvalue_yaw_2) false)
  (`SceneComponent.SetVisibility` (`Actor.RootComponent` (`self.WidgetActor`)) true false)
  (`self.K2_AttachToComponent` (`self.WidgetActor`) (`self.ReplicatedVRCamera`) "None" "KeepWorld" "KeepWorld" "KeepWorld" false))

(fn `UpdateWizardTransform`
  (bind _returnvalue (`SceneComponent.K2_GetComponentToWorld` (`self.ReplicatedVRCamera`)))
  (bind _returnvalue_2 (`SceneComponent.K2_GetComponentToWorld` (`self.Character_Wizard_01`)))
  (`SceneComponent.K2_SetWorldLocationAndRotation` (`self.Character_Wizard_01`) (`KismetMathLibrary.MakeVector` (.x (.location _returnvalue)) (.y (.location _returnvalue)) (.z (.location _returnvalue_2))) (`KismetMathLibrary.MakeRotator` (.roll (.rotation _returnvalue_2)) (.pitch (.rotation _returnvalue_2)) (- (.yaw (.rotation _returnvalue)) 90.0)) false false))

(fn `UserConstructionScript`
  (set `self.VRBounds` (`SteamVRChaperoneComponent.GetBounds` (`self.SteamVRChaperone`))))