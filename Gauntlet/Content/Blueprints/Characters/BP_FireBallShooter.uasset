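; BP_FireBallShooter is an actor that periodically launches BP_Fireball actors along its arrow component's forward direction.
; After a random startup delay that follows BeginPlay, a looping timer fires at a fixed interval.
; Each tick spawns a fireball at the shooter's location only while IsShooting is set, then passes it the arrow's direction as initial velocity.
; IsShootingMaxFireball selects a slightly enlarged fireball instead of a normal-sized one.
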(event `self.ReceiveBeginPlay`
  (`KismetSystemLibrary.Delay` (`KismetMathLibrary.RandomFloatInRange` 3.0 4.0))
  (`KismetSystemLibrary.K2_SetTimerDelegate` (delegate `ShootRandomFireball`) 3.0 true))

(event `ShootRandomFireball`
  (bind _returnvalue (`self.K2_GetActorLocation`))
  (bind _returnvalue_2 (`KismetMathLibrary.Normal` (`SceneComponent.GetForwardVector` (`self.Arrow`))))
  (if (`self.IsShooting`)
    (if (`self.IsShootingMaxFireball`)
      (bind _returnvalue_3 (`|SpawnActorFromClass` "/Game/Blueprints/GestureSpells/Spells/BP_Fireball.BP_Fireball_C" (`KismetMathLibrary.MakeTransform` _returnvalue (struct) (* (`KismetMathLibrary.Normal` (`KismetMathLibrary.MakeVector` 1.0 1.0 1.0)) 2)) "Undefined" "OverrideRootScale" null null))
      (`/Game/Blueprints/GestureSpells/Spells/BP_Fireball.SetInitialVelocity` _returnvalue_3 _returnvalue_2)
      (else
        (bind _returnvalue_4 (`|SpawnActorFromClass` "/Game/Blueprints/GestureSpells/Spells/BP_Fireball.BP_Fireball_C" (`KismetMathLibrary.MakeTransform` _returnvalue) "Undefined" "OverrideRootScale" null null))
        (`/Game/Blueprints/GestureSpells/Spells/BP_Fireball.SetInitialVelocity` _returnvalue_4 _returnvalue_2)))))

(fn `UserConstructionScript`)