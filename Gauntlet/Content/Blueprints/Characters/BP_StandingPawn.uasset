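; VR standing pawn with floor-origin tracking, LAN multiplayer session controls and a simple hit-point counter.
; Host input creates a session and opens Gym as a listen server, while Join input joins the first session found.
; The W key removes a hit point, updates the health text and quits at zero.
; Tick prints changed headset and controller positions; ShowMenuWidget only spawns a menu actor, leaving its placement logic unconnected.
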(event `InputAction|Host`
  (params (Key :type "Key Structure"))
  ;[1 1 1] Host Session
  (:`Pressed`
    (`CreateSessionCallbackProxy.CreateSession` (`GameplayStatics.GetPlayerController` 0) 10 true
      (:`OnSuccess`
        (`GameplayStatics.OpenLevel` "Gym" true "listen"))
      (:`OnFailure`
        (`KismetSystemLibrary.PrintString` "Failed")))))

(event `InputAction|Join`
  (params (Key :type "Key Structure"))
  ;[1 1 1] Join Session
  (:`Pressed`
    (`KismetSystemLibrary.PrintString` "Searching sessions..." true true (struct :`G` 0.66 :`B` 1.0 :`A` 1.0) 10.0)
    (bind _results (`FindSessionsCallbackProxy.FindSessions` (`GameplayStatics.GetPlayerController` 0) 10 true)
      (:`OnSuccess`
        (bind _output (`|GetArrayItem` _results))
        (`KismetSystemLibrary.PrintString` (`KismetStringLibrary.Concat_StrStr` "Found session: " (`FindSessionsCallbackProxy.GetServerName` _output)) true true (struct :`G` 0.66 :`B` 1.0 :`A` 1.0) 10.0)
        (`JoinSessionCallbackProxy.JoinSession` (`GameplayStatics.GetPlayerController` 0) _output
          (:`OnSuccess`
            (`KismetSystemLibrary.PrintString` "Joined session" true true (struct :`G` 0.66 :`B` 1.0 :`A` 1.0) 10.0))
          (:`OnFailure`
            (`KismetSystemLibrary.PrintString` "Failed to join session" true true (struct :`R` 1.0 :`G` 0.006241 :`A` 1.0) 10.0))))
      (:`OnFailure`
        (`KismetSystemLibrary.PrintString` "Error while trying to find sessions" true true (struct :`R` 1.0 :`B` 0.035091 :`A` 1.0) 10.0)))))

(event `self.ReceiveBeginPlay`
  ;[1 1 1] Set Character Start Attributes
  (`HeadMountedDisplayFunctionLibrary.SetTrackingOrigin` "Floor")
  (bind _output_get (set `self.HitPoints` 3))
  (`TextRenderComponent.K2_SetText` (`self.HealthText`) (`KismetTextLibrary.Conv_IntToText` _output_get)))

(event `self.ReceiveTick`
  (params (DeltaSeconds :type "Float (single-precision)"))
  (bind _returnvalue (`KismetStringLibrary.Concat_StrStr` "Camera:" (`KismetStringLibrary.Conv_VectorToString` (`SceneComponent.K2_GetComponentLocation` (`self.VRCamera`))) "_Left:" (`KismetStringLibrary.Conv_VectorToString` (`SceneComponent.K2_GetComponentLocation` (`self.MC_Left`))) "Right:" (`KismetStringLibrary.Conv_VectorToString` (`SceneComponent.K2_GetComponentLocation` (`self.MC_Right`)))))
  ;[1 1 1] Print debug data
  (if (`KismetStringLibrary.NotEqual_StrStr` _returnvalue (`self.Positions`))
    (bind _output_get (set `self.Positions` _returnvalue))
    (`KismetSystemLibrary.PrintString` _output_get true true (struct :`G` 0.66 :`B` 1.0 :`A` 1.0) 0.1)))

(event `Key|W`
  (params (Key :type "Key Structure"))
  ;[1 1 1] Apply Damage
  (:`Pressed`
    (bind _result (`/Engine/EditorBlueprintResources/StandardMacros.DecrementInt` (`self.Hitpoints`))
      (:`  `
        (bind _output_get (set `self.Hitpoints` _result))
        ;;[1 1 1] Update Health UI
        (`TextRenderComponent.K2_SetText` (`self.HealthText`) (`KismetTextLibrary.Conv_IntToText` _output_get))
        ;;[1 1 1] End Game
        (if (<= _output_get 0)
          (`KismetSystemLibrary.QuitGame` null "Quit"))))))

(fn `ShowMenuWidget`
  (bind _returnvalue (`|SpawnActorFromClass` "/Game/Blueprints/Widgets/BP_MenuActor.BP_MenuActor_C" (`KismetMathLibrary.MakeTransform` (0.0 0.0 0.0) (struct) (0.1 0.1 0.1)) "Undefined" "OverrideRootScale" null null))
  (cast `/Game/Blueprints/Widgets/BP_MenuActor` _returnvalue))

(fn `UserConstructionScript`)