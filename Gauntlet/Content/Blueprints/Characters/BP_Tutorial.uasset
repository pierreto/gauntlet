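; Tutorial controller that teaches fireball and shield gestures to the nearest BP_Hands, then opens the Arena level as a listen server.
; A Tick-driven state machine loops replayer recordings per lesson, while TargetDestroyed toggles hands and shooter between lessons.
; As wired, Begin waits two seconds and jumps to Transition, skipping both lessons because the Fireball entry is disconnected.
; Transition thickens exponential fog at accelerating speed until End loads the level.
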(event `self.ReceiveBeginPlay`
  (bind _shieldtarget (`self.ShieldTarget`))
  (`|ExecutionSequence`
    (:`then_0`
      (bind _asbp_replayer (cast `/Game/Blueprints/Dev/Record/BP_Replayer` (`ChildActorComponent.ChildActor` (`self.ReplayerActor`))))
      (bind _output_get (set `self.Replayer` _asbp_replayer))
      (set `/Game/Blueprints/Dev/Record/BP_Replayer.RecognizeGesture` false _output_get)
      (bind (_recordings _success) (`/Game/Blueprints/Dev/Record/BP_Replayer.LoadRecording` _output_get "FireballRecordings"))
      (if _success
        (set `self.FireballRecordings` _recordings)
        (bind (_recordings_2 _success_2) (`/Game/Blueprints/Dev/Record/BP_Replayer.LoadRecording` (`self.Replayer`) "ShieldRecordings"))
        (if _success_2
          (set `self.ShieldRecordings` _recordings_2)
          (`SceneComponent.SetVisibility` _shieldtarget false true)
          (bind _asbp_tutorial_target (cast `/Game/Blueprints/Characters/BP_TutorialTarget` (`ChildActorComponent.ChildActor` _shieldtarget)))
          (set `/Game/Blueprints/Characters/BP_TutorialTarget.IsInvicible` true _asbp_tutorial_target)
          (bind _closestbphands (`self.GetClosestBpHands`))
          (bind _output_get_2 (set `self.Hands` _closestbphands))
          (set `/Game/Blueprints/Characters/BP_Hands.Invincible` true _output_get_2)
          (set `/Game/Blueprints/GestureSpells/Hand.ActivateLeft` false (`/Game/Blueprints/Characters/BP_Hands.HandL` _output_get_2))
          (set `self.TutorialState` "NewEnumerator3")
          (else
            (`KismetSystemLibrary.PrintString` "Failed to shield recording!" true true (struct :`R` 1.0 :`A` 1.0))))
        (else
          (`KismetSystemLibrary.PrintString` "Failed to fireball recording!" true true (struct :`R` 1.0 :`A` 1.0)))))
    (:`then_1`
      ;[1 1 1] Get exponential fog
      (bind _outactors (`GameplayStatics.GetAllActorsOfClass` "/Script/Engine.ExponentialHeightFog"))
      (if (> (`KismetArrayLibrary.Array_Length` _outactors) 0)
        (set `self.ExponentialFog` (`ExponentialHeightFog.Component` (`|GetArrayItem` _outactors)))))))

(event `self.ReceiveTick`
  (params (DeltaSeconds :type "Float (single-precision)"))
  (set `self.CurrentDelta` DeltaSeconds)
  (switch `/Game/Blueprints/Characters/ETutorialStates` (`self.TutorialState`)
    (:`NewEnumerator3`
      (`KismetSystemLibrary.Delay` 2.0)
      (set `self.TutorialState` "NewEnumerator6"))
    (:`NewEnumerator0`
      ;[1 1 1] Loop on firenall recordings
      (`self.LoopRecording` (`self.FireballRecordings`)))
    (:`NewEnumerator4`
      ;[1 1 1] Loop on shield recordings
      (`self.LoopRecording` (`self.ShieldRecordings`)))
    (:`NewEnumerator6`
      (bind _done (`self.IncreaseFogDensity` (`self.CurrentDelta`)))
      (if _done
        (set `self.TutorialState` "NewEnumerator2")))
    (:`NewEnumerator2`
      (set `/Game/Blueprints/Characters/BP_Hands.Invincible` false (`self.Hands`))
      (if (`self.IsServer`)
        _
        (else
          _))
      (`GameplayStatics.OpenLevel` "Arena" true "listen"))))

(event `TargetDestroyed`
  (bind _shieldtarget (`self.ShieldTarget`))
  (bind _heldfireball (`/Game/Blueprints/GestureSpells/Hand.HeldFireball` (`/Game/Blueprints/Characters/BP_Hands.HandR` (`self.Hands`))))
  (switch `/Game/Blueprints/Characters/ETutorialStates` (`self.TutorialState`)
    (:`NewEnumerator0`
      (`/Game/Blueprints/Dev/Record/BP_Replayer.Stop` (`self.Replayer`))
      (bind _asbp_fire_ball_shooter (cast `/Game/Blueprints/Dev/BP_FireBallShooter` (`ChildActorComponent.ChildActor` (`self.FireballShooter`))))
      (set `/Game/Blueprints/Dev/BP_FireBallShooter.IsShooting` true _asbp_fire_ball_shooter)
      (`SceneComponent.SetVisibility` _shieldtarget true true)
      (bind _asbp_tutorial_target (cast `/Game/Blueprints/Characters/BP_TutorialTarget` (`ChildActorComponent.ChildActor` _shieldtarget)))
      (set `/Game/Blueprints/Characters/BP_TutorialTarget.IsInvicible` false _asbp_tutorial_target)
      (set `/Game/Blueprints/GestureSpells/Hand.ActivateLeft` true (`/Game/Blueprints/Characters/BP_Hands.HandL` (`self.Hands`)))
      (set `/Game/Blueprints/GestureSpells/Hand.ActivateRight` false (`/Game/Blueprints/Characters/BP_Hands.HandR` (`self.Hands`)))
      (if (`KismetSystemLibrary.IsValid` _heldfireball)
        (`self.K2_DestroyActor` _heldfireball))
      (set `self.TutorialState` "NewEnumerator4"))
    (:`NewEnumerator4`
      (`KismetSystemLibrary.PrintString` "FireballDeflected")
      (`/Game/Blueprints/Dev/Record/BP_Replayer.Stop` (`self.Replayer`))
      (bind _asbp_fire_ball_shooter_2 (cast `/Game/Blueprints/Dev/BP_FireBallShooter` (`ChildActorComponent.ChildActor` (`self.FireballShooter`))))
      (set `/Game/Blueprints/Dev/BP_FireBallShooter.IsShooting` false _asbp_fire_ball_shooter_2)
      (set `/Game/Blueprints/GestureSpells/Hand.ActivateRight` true (`/Game/Blueprints/Characters/BP_Hands.HandR` (`self.Hands`)))
      (set `self.TutorialState` "NewEnumerator2"))))

(fn `GetClosestBpHands`
  (returns (ClosestBPHands :type "/Game/Blueprints/Characters/BP_Hands Object Reference"))
  (locals (MinDistanceHand :type "Float (double-precision)" :default 9999.0) (ClosestHands :type "/Game/Blueprints/Characters/BP_Hands Object Reference"))
  (bind _outactors (`GameplayStatics.GetAllActorsOfClass` "/Game/Blueprints/Characters/BP_Hands.BP_Hands_C"))
  (for _array_element _outactors
    (bind _returnvalue (`KismetMathLibrary.VSize` (- (`SceneComponent.K2_GetComponentLocation` (`Actor.RootComponent` _array_element)) (`SceneComponent.K2_GetComponentLocation` (`self.DefaultSceneRoot`)))))
    (if (< _returnvalue (`local.MinDistanceHand`))
      (set `local.MinDistanceHand` _returnvalue)
      (set `local.ClosestHands` _array_element)))
  (return (`local.ClosestHands`)))

(fn `GetFogSpeed`
  (params (DeltaTime :type "Float (double-precision)"))
  (returns (Speed :type "Float (double-precision)"))
  (bind _output_get (set `self.FogSpeed` (+ (`self.FogSpeed`) (* (`self.FogAcceleration`) DeltaTime))))
  (return _output_get))

(fn `GetServerIP`
  (returns (IP :type String))
  (locals (_IP :type String))
  (bind _returnvalue (`KismetSystemLibrary.GetCommandLine`))
  (bind (_lefts _rights) (`KismetStringLibrary.Split` _returnvalue "ip="))
  (bind (_lefts_2 _rights_2 _returnvalue_2) (`KismetStringLibrary.Split` _rights " "))
  (if _returnvalue_2
    (set `local._IP` _lefts_2)
    (else
      (set `local._IP` _rights)))
  (return (`local._IP`)))

(fn `IncreaseFogDensity`
  (params (DeltaTime :type "Float (double-precision)"))
  (returns (Done :type Boolean))
  (bind _exponentialfog (`self.ExponentialFog`))
  (`/Engine/EditorBlueprintResources/StandardMacros.IsValid` _exponentialfog
    (:`Is Valid`
      (`ExponentialHeightFogComponent.SetFogDensity` _exponentialfog (+ (`ExponentialHeightFogComponent.FogDensity` _exponentialfog) (* (`self.GetFogSpeed` DeltaTime) DeltaTime)))
      (return (>= (`ExponentialHeightFogComponent.FogDensity` (`self.ExponentialFog`)) (`self.MaxFogDensity`))))))

(fn `IsServer`
  (returns (IsServer :type Boolean))
  (bind _returnvalue (`KismetSystemLibrary.GetCommandLine`))
  (return (`KismetStringLibrary.Contains` _returnvalue "server")))

(fn `LoopRecording`
  (params (Recordings :type "Array of /Game/Blueprints/Dev/Record/GestureRecording Structure"))
  (if (not (`/Game/Blueprints/Dev/Record/BP_Replayer.IsPlayingRecording` (`self.Replayer`)))
    (bind _output_get (set `self.Recordings` Recordings))
    (`/Game/Blueprints/Dev/Record/BP_Replayer.Play` (`self.Replayer`) _output_get)))

(fn `UserConstructionScript`)