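; VR wizard arena character that conjures and throws fireballs and tracks hit points.
; Tick buffers hand velocities and moves the owner-hidden wizard mesh with the headset's position and yaw.
; A server-spawned fireball attaches to the right controller; shooting replaces it with one launched at twice the averaged hand velocity.
; Damage updates health text and removes a health-point actor; the GameMode's game-ended event shows Victory or Defeat by remaining HP.
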(event `self.ReceiveBeginPlay`
  ;[1 1 1] Set Character Start Attributes
  (bind _asbp_gym_game_mode (cast `/Game/Blueprints/Gameplay/BP_GymGameMode` (`GameplayStatics.GetGameMode`)))
  (add `/Game/Blueprints/Gameplay/BP_GymGameMode.OnGameEnded` _asbp_gym_game_mode (delegate `GameEnded`))
  (`HeadMountedDisplayFunctionLibrary.SetTrackingOrigin` "Floor")
  (bind _output_get (set `self.HitPoints` 3.0))
  (`TextRenderComponent.K2_SetText` (`self.HealthText`) (`KismetTextLibrary.Conv_DoubleToText` _output_get "HalfToEven"))
  (`PrimitiveComponent.SetOwnerNoSee` (`self.Character_Wizard_01`) true)
  (`/Engine/EditorBlueprintResources/ActorMacros.Switch Has Authority`
    (:`Authority`
      (`self.CreateHPActors`))))

(event `self.ReceiveTick`
  (params (DeltaSeconds :type "Float (single-precision)"))
  ;[1 1 1] Print debug data
  ;;[1 1 1] Store Velocity and Print on Screen
  (`|ExecutionSequence`
    (:`then_0`
      (`self.StoreRightHandVelocity`)
      (`self.StoreLeftHandVelocity`)
      (if (>= (`KismetMathLibrary.VSize` (`self.GetRightHandVelocity`)) 100.0)
        _))
    (:`then_1`
      (`self.UpdateCharacterTransform`))))

(event `GameEnded`
  (`self.ShowEndGameClient`))

(event `ShowEndGameClient`
  (`self.CreateEndGameWidget` (<= (`self.HitPoints`) 0.0)))

(event `self.ReceiveAnyDamage`
  (params (Damage :type "Float (single-precision)") (DamageType :type "DamageType Object Reference") (InstigatedBy :type "Controller Object Reference") (DamageCauser :type "Actor Object Reference"))
  ;[1 1 1] Apply Damage
  (bind _output_get (set `self.HitPoints` (- (`self.HitPoints`) Damage)))
  ;;[1 1 1] Update Health UI
  (`TextRenderComponent.K2_SetText` (`self.HealthText`) (`KismetTextLibrary.Conv_DoubleToText` _output_get "HalfToEven"))
  (`self.DestroyHPActors`)
  ;;[1 1 1] End Game
  (if (<= _output_get 0.0)
    _))

(event `SpawnFireball`
  ;[1 1 1] Spawn Fireball on Server
  (`/Engine/EditorBlueprintResources/ActorMacros.Switch Has Authority`
    (:`Authority`
      (bind _returnvalue (`|SpawnActorFromClass` (`self.SpellToSpawn`) (`SceneComponent.K2_GetComponentToWorld` (`self.SM_Right`)) "AlwaysSpawn" "OverrideRootScale" null self))
      (bind _output_get (set `self.HeldFireBall` _returnvalue))
      (`self.AttachFireball` (`/Game/Blueprints/GestureSpells/Spells/BP_Fireball.Fire Ball` _output_get)))))

(event `AttachFireball`
  (params (Target :type "SceneComponent Object Reference"))
  ;[1 1 1] Spawn Fireball on Server
  (`SceneComponent.K2_AttachToComponent` Target (`self.RightMotionController`) "None" "KeepRelative" "KeepRelative" "KeepRelative" false))

(event `ShootFireBall`
  ;[1 1 1] Shoot Fireball on Server
  (`self.ShootFireBallMulti`))

(event `ShootFireBallMulti`
  (bind _heldfireball (`self.HeldFireball`))
  ;[1 1 1] Shoot Fireball on Server
  (if (`KismetSystemLibrary.IsValid` _heldfireball)
    (`self.K2_DestroyActor` _heldfireball)
    (bind _returnvalue (`|SpawnActorFromClass` (`self.SpellToSpawn`) (`SceneComponent.K2_GetComponentToWorld` (`self.SM_Right`)) "AlwaysSpawn" "OverrideRootScale" null self))
    (`/Game/Blueprints/GestureSpells/Spells/BP_Fireball.SetVelocity` _returnvalue (* (`self.GetRightHandVelocity`) 2))))

(event `InputAction|Spawn Fireball`
  (params (Key :type "Key Structure"))
  ;[1 1 1] Handle Input
  (:`Pressed`
    (`self.SpawnFireball`)))

(event `InputAction|ShootFireBall`
  (params (Key :type "Key Structure"))
  ;[1 1 1] Handle Input
  (:`Pressed`
    (`self.ShootFireBall`)))

(event `InputAction|Exit`
  (params (Key :type "Key Structure"))
  ;[1 1 1] Handle Input
  (:`Pressed`
    (`KismetSystemLibrary.QuitGame` null "Quit")))

(fn `CreateEndGameWidget`
  (params (HasLost :type Boolean))
  (bind _returnvalue (`GameplayStatics.GetPlayerController` 0))
  (`/Engine/EditorBlueprintResources/ActorMacros.Switch Has Authority`
    (:`Authority`
      _)
    (:`Remote`
      _))
  (if HasLost
    (bind _returnvalue_2 (`|CreateWidget` "/Game/Assets/Widgets/Defeat.Defeat_C" _returnvalue))
    (else
      (bind _returnvalue_3 (`|CreateWidget` "/Game/Assets/Widgets/Victory.Victory_C" _returnvalue))))
  (`UserWidget.AddToViewport` _returnvalue_2 0)
  (`UserWidget.AddToViewport` _returnvalue_3 0))

(fn `CreateHPActors`
  (bind _character_wizard_01 (`self.Character_Wizard_01`))
  (bind _returnvalue (`SceneComponent.GetUpVector` _character_wizard_01))
  (bind _output_get (set `self.HitPoints` (`self.HitPoints`)))
  (for _index (range 1 (+ (`KismetMathLibrary.FTrunc` _output_get) 1))
    (bind _returnvalue_2 (`|SpawnActorFromClass` "/Game/Blueprints/BP_HealthPoint.BP_HealthPoint_C" (`KismetMathLibrary.MakeTransform` (0.0 0.0 0.0)) "AlwaysSpawn" "OverrideRootScale" null null))
    (`self.K2_SetActorLocation` _returnvalue_2 (+ (`SceneComponent.K2_GetComponentLocation` _character_wizard_01) (* _returnvalue 20) (* _returnvalue (* _index (`self.HorizontalHpOffset`))) (* _returnvalue (/ (* (+ _output_get 1.0) (`self.HorizontalHpOffset`)) -2.0)) (150.0 150.0 0.0)) false false)
    (`KismetArrayLibrary.Array_Add` (`self.HpActors`) _returnvalue_2)))

(fn `DestroyHPActors`
  (bind _returnvalue (- (`KismetArrayLibrary.Array_Length` (`self.HpActors`)) 1))
  (`self.K2_DestroyActor` (`|GetArrayItem` (`self.HpActors`) _returnvalue))
  (`KismetArrayLibrary.Array_Remove` (`self.HpActors`) _returnvalue))

(fn `GetLeftHandVelocity`
  (returns (Average :type "Vector Structure"))
  (return (`KismetMathLibrary.GetVectorArrayAverage` (`self.LeftHandVelocities`))))

(fn `GetRightHandVelocity`
  (returns (Average :type "Vector Structure"))
  (return (`KismetMathLibrary.GetVectorArrayAverage` (`self.RightHandVelocities`))))

(fn `StoreLeftHandVelocity`
  (bind _lefthandvelocities (`self.LeftHandVelocities`))
  ;[1 1 1] Store Left Hand Velocity To Compute Average Later
  (bind _returnvalue (`PrimitiveComponent.GetPhysicsLinearVelocity` (`self.SM_Left`) "None"))
  (`KismetArrayLibrary.Array_Add` _lefthandvelocities _returnvalue)
  (if (>= (`KismetArrayLibrary.Array_Length` _lefthandvelocities) 10)
    (`KismetArrayLibrary.Array_Remove` (`self.LeftHandVelocities`))))

(fn `StoreRightHandVelocity`
  (bind _righthandvelocities (`self.RightHandVelocities`))
  ;[1 1 1] Store Right Hand Velocity To Compute Average Later
  (bind _returnvalue (`PrimitiveComponent.GetPhysicsLinearVelocity` (`self.SM_Right`) "None"))
  (`KismetArrayLibrary.Array_Add` _righthandvelocities _returnvalue)
  (if (>= (`KismetArrayLibrary.Array_Length` _righthandvelocities) 10)
    (`KismetArrayLibrary.Array_Remove` (`self.RightHandVelocities`))))

(fn `UpdateCharacterTransform`
  (bind _returnvalue (`SceneComponent.K2_GetComponentToWorld` (`self.VRReplicatedCamera`)))
  (bind _returnvalue_2 (`SceneComponent.K2_GetComponentToWorld` (`self.Character_Wizard_01`)))
  (`SceneComponent.K2_SetWorldLocationAndRotation` (`self.Character_Wizard_01`) (`KismetMathLibrary.MakeVector` (.x (.location _returnvalue)) (.y (.location _returnvalue)) (.z (.location _returnvalue_2))) (`KismetMathLibrary.MakeRotator` (.roll (.rotation _returnvalue_2)) (.pitch (.rotation _returnvalue_2)) (- (.yaw (.rotation _returnvalue)) 90.0)) false false))

(fn `UserConstructionScript`)