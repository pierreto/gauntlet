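; BP_Character is a VR player character with a small hit point pool shown on a health text display.
; BeginPlay sets floor-level tracking and initializes health.
; Tick prints camera and both motion controller world positions as debug text whenever they change.
; Pressing W removes a hit point, refreshes the health text and quits the game when none remain.
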(event `self.ReceiveBeginPlay`
  ;[1 1 1] Set Character Start Attributes
  (`HeadMountedDisplayFunctionLibrary.SetTrackingOrigin` "Floor")
  (bind _output_get (set `self.HitPoints` 3))
  (`TextRenderComponent.K2_SetText` (`self.HealthText`) (`KismetTextLibrary.Conv_IntToText` _output_get)))

(event `self.ReceiveTick`
  (params (DeltaSeconds :type "Float (single-precision)"))
  (bind _returnvalue (`KismetStringLibrary.Concat_StrStr` "Camera:" (`KismetStringLibrary.Conv_VectorToString` (`SceneComponent.K2_GetComponentLocation` (`self.VRReplicatedCamera`))) "_Left:" (`KismetStringLibrary.Conv_VectorToString` (`SceneComponent.K2_GetComponentLocation` (`self.LeftMotionController`))) "Right:" (`KismetStringLibrary.Conv_VectorToString` (`SceneComponent.K2_GetComponentLocation` (`self.RightMotionController`)))))
  ;[1 1 1] Print debug data
  (if (`KismetStringLibrary.NotEqual_StrStr` _returnvalue (`self.Positions`))
    (bind _output_get (set `self.Positions` _returnvalue))
    (`KismetSystemLibrary.PrintString` _output_get true true (struct :`G` 0.66 :`B` 1.0 :`A` 1.0) 0.1)))

(event `Key|W`
  (params (Key :type "Key Structure"))
  ;[1 1 1] Apply Damage
  (:`Pressed`
    (bind _result (`/Engine/EditorBlueprintResources/StandardMacros.DecrementInt` (`self.Hitpoints`))
      (:`  `
        (bind _output_get (set `self.Hitpoints` _result))
        ;;[1 1 1] Update Health UI
        (`TextRenderComponent.K2_SetText` (`self.HealthText`) (`KismetTextLibrary.Conv_IntToText` _output_get))
        ;;[1 1 1] End Game
        (if (<= _output_get 0)
          (`KismetSystemLibrary.QuitGame` null "Quit"))))))

(fn `UserConstructionScript`)