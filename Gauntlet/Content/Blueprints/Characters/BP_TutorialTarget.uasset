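; BP_TutorialTarget is a destructible target for the tutorial that reports its destruction to its parent BP_Tutorial actor.
; Any damage lowers its HitPoint unless IsInvicible is set.
; At zero or below, it casts its parent actor to BP_Tutorial, calls TargetDestroyed and destroys itself.
; If that cast fails, the target is not destroyed.
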(event `self.ReceiveAnyDamage`
  (params (Damage :type "Float (single-precision)") (DamageType :type "DamageType Object Reference") (InstigatedBy :type "Controller Object Reference") (DamageCauser :type "Actor Object Reference"))
  (if (not (`self.IsInvicible`))
    (bind _output_get (set `self.HitPoint` (- (`self.HitPoint`) Damage)))
    (if (<= _output_get 0.0)
      (bind _asbp_tutorial (cast `/Game/Blueprints/Characters/BP_Tutorial` (`self.GetParentActor`)))
      (`/Game/Blueprints/Characters/BP_Tutorial.TargetDestroyed` _asbp_tutorial)
      (`self.K2_DestroyActor`))))

(fn `UserConstructionScript`)