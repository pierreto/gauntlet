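; BP_FireBallShooter is an actor in the Dev folder that periodically fires BP_Fireball projectiles along the forward direction of its Arrow component.
; A random delay of up to a second on BeginPlay offsets the start of a looping timer.
; Each tick of that timer checks IsShooting, spawns a fireball at a slightly jittered point around the actor and passes it the normalized Arrow direction as initial velocity.
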(event `self.ReceiveBeginPlay`
  (`KismetSystemLibrary.Delay` (`KismetMathLibrary.RandomFloatInRange` 0.0 1.0))
  (`KismetSystemLibrary.K2_SetTimerDelegate` (delegate `ShootRandomFireball`) 3.0 true))

(event `ShootRandomFireball`
  (if (`self.IsShooting`)
    (bind _returnvalue (`|SpawnActorFromClass` "/Game/Blueprints/GestureSpells/Spells/BP_Fireball.BP_Fireball_C" (`KismetMathLibrary.MakeTransform` (`KismetMathLibrary.RandomPointInBoundingBox` (`self.K2_GetActorLocation`) (2.0 2.0 2.0))) "Undefined" "OverrideRootScale" null null))
    (`/Game/Blueprints/GestureSpells/Spells/BP_Fireball.SetInitialVelocity` _returnvalue (`KismetMathLibrary.Normal` (`SceneComponent.GetForwardVector` (`self.Arrow`))))))

(fn `UserConstructionScript`)