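; Dev VR recorder that captures two-handed gesture recordings into a RecordingSaveGame.
; Recording toggles on an input action or when both fists close well below the head, edge-triggered by the SwitchToggle macro.
; While recording, each tick stores both hand pose snapshots, elapsed time and transforms with camera-offset locations, drawing debug spheres at the hands.
; Stopping saves the frames to the save slot and clears the buffer.
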(event `self.ReceiveBeginPlay`
  ;[1 1 1] Set tracking origin
  (`HeadMountedDisplayFunctionLibrary.SetTrackingOrigin` "Floor"))

(event `self.ReceiveTick`
  (params (DeltaSeconds :type "Float (single-precision)"))
  ;[1 1 1] Record gesture
  (`|ExecutionSequence`
    (:`then_0`
      (`self.SwitchToggle`
        (:`On`
          (`self.ToggleRecording`))))
    (:`then_1`
      (if (`self.IsRecording`)
        (`self.Record` DeltaSeconds)))))

(event `InputAction|RecordGesture`
  (params (Key :type "Key Structure"))
  ;[1 1 1] Start and stop recording from keyboard
  (:`Released`
    (`self.ToggleRecording`)))

(event `InputAction|Exit`
  (params (Key :type "Key Structure"))
  ;[1 1 1] Quit
  (:`Pressed`
    (`KismetSystemLibrary.QuitGame` null "Quit")))

(fn `DetectRecordingPostion`
  (returns (Detected :type Boolean))
  (bind (_returnvalue_x _returnvalue_y _returnvalue_z) (`KismetMathLibrary.BreakVector` (`SceneComponent.K2_GetComponentLocation` (`self.SkeletalMeshL`))))
  (bind (_returnvalue_x_2 _returnvalue_y_2 _returnvalue_z_2) (`KismetMathLibrary.BreakVector` (`SceneComponent.K2_GetComponentLocation` (`self.SkeletalMeshR`))))
  (bind (_returnvalue_x_3 _returnvalue_y_3 _returnvalue_z_3) (`KismetMathLibrary.BreakVector` (`SceneComponent.K2_GetComponentLocation` (`self.Camera`))))
  (bind _isclosed (`/Game/Blueprints/GestureSpells/Hand.IsFistClosed` (`self.LeftHand`)))
  (bind _isclosed_2 (`/Game/Blueprints/GestureSpells/Hand.IsFistClosed` (`self.RightHand`)))
  (return (and _isclosed_2 _isclosed (>= (- _returnvalue_z_3 _returnvalue_z) 30.0) (>= (- _returnvalue_z_3 _returnvalue_z_2) 30.0))))

(fn `GetRelativeTransform`
  (params (Component :type "SceneComponent Object Reference"))
  (returns (Transform :type "Transform Structure"))
  (return (`KismetMathLibrary.MakeTransform` (- (.location (`SceneComponent.K2_GetComponentToWorld` Component)) (`SceneComponent.K2_GetComponentLocation` (`self.Camera`))) (.rotation (`SceneComponent.K2_GetComponentToWorld` Component)) (.scale (`SceneComponent.K2_GetComponentToWorld` Component)))))

(fn `Record`
  (params (DeltaSeconds :type "Float (double-precision)"))
  (locals (Delta :type "Float (double-precision)") (LeftPose :type "PoseSnapshot Structure") (RightPose :type "PoseSnapshot Structure"))
  (bind _leftpose (`local.LeftPose`))
  (bind _rightpose (`local.RightPose`))
  (bind _output_get (set `local.Delta` DeltaSeconds))
  (set `self.CurrentRecordTime` (+ _output_get (`self.CurrentRecordTime`)))
  (`KismetSystemLibrary.DrawDebugSphere` (`SceneComponent.K2_GetComponentLocation` (`self.SkeletalMeshR`)) 10.0 12 (struct :`R` 1.0 :`A` 1.0) -1.0)
  (`KismetSystemLibrary.DrawDebugSphere` (`SceneComponent.K2_GetComponentLocation` (`self.SkeletalMeshL`)) 10.0 12 (struct :`R` 1.0 :`A` 1.0) -1.0)
  (`SkeletalMeshComponent.SnapshotPose` (`self.SkeletalMeshL`) _leftpose)
  (`SkeletalMeshComponent.SnapshotPose` (`self.SkeletalMeshR`) _rightpose)
  (`KismetArrayLibrary.Array_Add` (`self.Recordings`) (make `/Game/Blueprints/Dev/Record/GestureRecording` _leftpose _rightpose (`self.GetRelativeTransform` (`self.SkeletalMeshL`)) (`self.GetRelativeTransform` (`self.SkeletalMeshR`)) (`self.CurrentRecordTime`))))

(fn `SaveRecording`
  (params (Recording :type "Array of /Game/Blueprints/Dev/Record/GestureRecording Structure"))
  (locals (Data :type "Array of String"))
  (`KismetSystemLibrary.PrintString` "Saving...")
  (bind _returnvalue (`GameplayStatics.CreateSaveGameObject` "/Game/Blueprints/Dev/Record/RecordingSaveGame.RecordingSaveGame_C"))
  (bind _output_get (set `/Game/Blueprints/Dev/Record/RecordingSaveGame.Recordings` Recording _returnvalue))
  (bind _returnvalue_2 (`GameplayStatics.SaveGameToSlot` _returnvalue (`/Game/Blueprints/Dev/Record/RecordingSaveGame.SlotName` _returnvalue) (`/Game/Blueprints/Dev/Record/RecordingSaveGame.UserIndex` _returnvalue)))
  (if _returnvalue_2
    (`KismetSystemLibrary.PrintString` (`KismetStringLibrary.Concat_StrStr` "Saved " (`KismetStringLibrary.Conv_IntToString` (`KismetArrayLibrary.Array_Length` _output_get)) " recordings!"))))

(fn `ToggleRecording`
  (bind _recordings (`self.Recordings`))
  (set `self.CurrentRecordTime` 0.0)
  (bind _output_get (set `self.IsRecording` (not (`self.IsRecording`))))
  (if (not _output_get)
    (`self.SaveRecording` _recordings))
  (`KismetArrayLibrary.Array_Clear` _recordings))

(fn `UserConstructionScript`
  (set `self.VRBounds` (`SteamVRChaperoneComponent.GetBounds` (`self.SteamVRChaperone`))))